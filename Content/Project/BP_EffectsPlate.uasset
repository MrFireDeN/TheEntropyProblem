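; BP_EffectsPlate is a plate actor that triggers a status effect when an actor implementing BPI_EffectsInterface overlaps it.
; A random switch selects among poison, regeneration, slowing, strength, weakness and max HP increase on BPEffectsComponent, some with debug prints.
; The random range is pinned to one value, so only Slowing runs.
; Slowing is the only call that receives the overlapping actor as target.
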(event EventBeginPlay)

(event Collision|EventActorBeginOverlap
  (params (OtherActor :type Actor%20Object%20Reference))
  (if (Utilities|DoesObjectImplementInterface OtherActor "/Game/Project/Blueprints/BPI_EffectsInterface.BPI_EffectsInterface_C")
    (switch int (Math|Random|RandomIntegerinRange 2 2)
      (:0
        (Development|PrintString "Отравление")
        (Default|Poison (Variables|Default|GetBP_EffectsComponent) 4 10))
      (:1
        (Development|PrintString "Регенерация")
        (Default|Regeneration (Variables|Default|GetBP_EffectsComponent) 3 5))
      (:2
        (Development|PrintString "Замедление")
        (Default|Slowing (Variables|Default|GetBP_EffectsComponent) 9.0 1e+01 OtherActor))
      (:3
        (Default|Strenght (Variables|Default|GetBP_EffectsComponent) 3.0 1e+01))
      (:4
        (Default|Weakness (Variables|Default|GetBP_EffectsComponent) 3.0 5.0)
        (Development|PrintString "Weakness"))
      (:5
        (Default|IncreasingtheMaxHp (Variables|Default|GetBP_EffectsComponent) 5.0 3e+01)))))

(event EventTick
  (params (DeltaSeconds :type Float%20%28single-precision%29)))

(fn ConstructionScript)