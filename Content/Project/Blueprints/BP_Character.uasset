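; Character Blueprint that handles smooth transitions between walking and running speeds.
; SetRunning switches TargetSpeed between WalkSpeed and RunSpeed, and BeginPlay starts it at WalkSpeed.
; Every Tick, SetSpeed uses FInterpTo to ease the Character Movement component's MaxWalkSpeed toward that target until they match.
; No input is bound here, and nothing in this file calls SetRunning.
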(event EventBeginPlay
  (Variables|Default|SetTarget%20Speed (Variables|Default|GetWalk%20Speed)))

(event Collision|EventActorBeginOverlap
  (params (OtherActor :type Actor%20Object%20Reference)))

(event EventTick
  (params (DeltaSeconds :type Float%20%28single-precision%29))
  (Utilities|SetSpeed DeltaSeconds))

(fn ConstructionScript)

(fn SetRunning
  (params (Is%20Run :type Boolean))
  (if Is%20Run
    (Variables|Default|SetTarget%20Speed (Variables|Default|GetRun%20Speed))
    (else
      (Variables|Default|SetTarget%20Speed (Variables|Default|GetWalk%20Speed)))))