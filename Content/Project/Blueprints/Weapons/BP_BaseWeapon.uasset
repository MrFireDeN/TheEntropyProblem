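; Base weapon actor, spawned as a child actor of BP_Character, that handles quick and strong melee attacks and stores weapon stats.
; Attack plays the current combo step's montage on the owner's mesh, updates BPCombatComponent and calls an empty ComboHandle hook.
; Montage end straightens the capsule, stops movement and clears hit actors; combo steps reset immediately, or after a retriggerable delay when interrupted.
; CalculateDamage scales health and stun damage by attack type and combo step.
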(event Custom|SetStats
  (params (HealthDamage :type Float%20%28double-precision%29) (StunDamage :type Float%20%28double-precision%29) (StaminaCost :type Float%20%28double-precision%29) (AttackRate :type Float%20%28double-precision%29) (AttackSphereRadius :type Float%20%28double-precision%29))
  (CallFunction|SetWeaponStats HealthDamage StunDamage StaminaCost AttackRate AttackSphereRadius))

(event Custom|Attack
  (params (AttackType :type E_AttackType%20Enum :default "NewEnumerator0"))
  ;[1 1 1] Attacking
  (Utilities|IsValid (Utilities|Array|Get(acopy) (Variables|Default|GetQuickAttackAnims) (Variables|Default|GetQuickComboStep))
    (:Is%20Valid
      (Utilities|IsValid (Utilities|Array|Get(acopy) (Variables|Default|GetStrongAttackAnims) (Variables|Default|GetStrongComboStep))
        (:Is%20Valid
          (Default|SetAttacking (Variables|Default|GetBP%20Combat%20Component) true)
          (Animation|Montage|PlayMontage (Variables|Default|GetMesh) (Utilities|Select :Index AttackType :NewEnumerator0 (Utilities|Array|Get(acopy) (Variables|Default|GetQuickAttackAnims) (Variables|Default|GetQuickComboStep)) :NewEnumerator1 (Utilities|Array|Get(acopy) (Variables|Default|GetStrongAttackAnims) (Variables|Default|GetStrongComboStep))) (Variables|Default|GetAttackRate)
            (:then
              (Variables|Default|SetLastAttackType AttackType)
              (CallFunction|ComboHandle))
            (:OnCompleted
              (Utilities|CharacterAnimCompleteHandle)
              (Default|ClearHitActors (Variables|Default|GetBP%20Combat%20Component))
              (Variables|Default|SetQuickComboStep 0 :!label _label)
              (Variables|Default|SetStrongComboStep 0)
              (Default|SetAttacking (Variables|Default|GetBP%20Combat%20Component) false))
            (:OnInterrupted
              (Utilities|CharacterAnimCompleteHandle)
              (Default|ClearHitActors (Variables|Default|GetBP%20Combat%20Component))
              (Utilities|FlowControl|RetriggerableDelay (Variables|Default|GetAttackRate))
              (goto _label))))))))

(event EventBeginPlay
  (bind _asbp_character (Utilities|Casting|CastToBP_Character (Actor|GetParentActor)))
  (bind _output_get (Variables|Default|SetAs%20BP%20Character _asbp_character))
  (Variables|Default|SetBP%20Combat%20Component (Variables|/Game/Project/Blueprints/Characters/BP_Character.BP_Character_C|GetBP_CombatComponent _output_get))
  (Variables|Default|SetMesh (Variables|/Script/Engine.Character|GetMesh _output_get)))

(event Collision|EventActorBeginOverlap
  (params (OtherActor :type Actor%20Object%20Reference)))

(event EventTick
  (params (DeltaSeconds :type Float%20%28single-precision%29)))

(fn ConstructionScript)

(fn SetWeaponStats
  (params (HealthDamage :type Float%20%28double-precision%29) (StunDamage :type Float%20%28double-precision%29) (StaminaCost :type Float%20%28double-precision%29) (AttackRate :type Float%20%28double-precision%29) (AttackSphereRadius :type Float%20%28double-precision%29))
  (Variables|Default|SetHealthDamage HealthDamage)
  (Variables|Default|SetStunDamage StunDamage)
  (Variables|Default|SetStaminaCost StaminaCost)
  (Variables|Default|SetAttackRate AttackRate)
  (Variables|Default|SetAttackSphereRadius AttackSphereRadius))

(fn GetWeaponStats
  (return (Variables|Default|GetHealthDamage) (Variables|Default|GetStunDamage) (Variables|Default|GetStaminaCost) (Variables|Default|GetAttackRate) (Variables|Default|GetAttackSphereRadius)))

(fn SetQuickAttackAnims
  (params (QucikAttackAnims :type Array%20of%20Anim%20Montage%20Object%20References))
  (Variables|Default|SetQuickAttackAnims QucikAttackAnims))

(fn SetStrongAttackAnims
  (params (StrongAttackAnims :type Array%20of%20Anim%20Montage%20Object%20References))
  (Variables|Default|SetStrongAttackAnims StrongAttackAnims))

(fn ComboHandle)

(fn CalculateDamage
  (bind _healthdamage (Variables|Default|GetHealthDamage))
  (Development|PrintString (Utilities|String|ToString(Float) _healthdamage))
  (return (Utilities|Select :Index (Variables|Default|GetLastAttackType) :NewEnumerator0 (+ _healthdamage (* (Variables|Default|GetQuickComboStep) 0.1)) :NewEnumerator1 (+ (* (Variables|Default|GetHealthDamage) 1.5) (* (Variables|Default|GetStrongComboStep) 0.3))) (Utilities|Select :Index (Variables|Default|GetLastAttackType) :NewEnumerator0 (+ (Variables|Default|GetStunDamage) (* (Variables|Default|GetQuickComboStep) 0.1)) :NewEnumerator1 (+ (* (Variables|Default|GetStunDamage) 1.5) (* (Variables|Default|GetStrongComboStep) 0.3)))))

(fn SetQuickComboStep
  (params (QuickComboStep :type Integer))
  (bind _output_get (Variables|Default|SetQuickComboStep (Math|Integer|Max(Integer) 0 QuickComboStep)))
  (return _output_get))

(fn SetStrongComboStep
  (params (StrongComboStep :type Integer))
  (bind _output_get (Variables|Default|SetStrongComboStep (Math|Integer|Max(Integer) 0 StrongComboStep)))
  (return _output_get))

(fn GetComboSteps
  (return (Variables|Default|GetQuickComboStep) (Variables|Default|GetStrongComboStep)))

(fn GetAttackAnimsCount
  (return (Utilities|Array|Length (Variables|Default|GetQuickAttackAnims)) (Utilities|Array|Length (Variables|Default|GetStrongAttackAnims))))