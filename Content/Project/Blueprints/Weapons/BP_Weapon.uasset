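; BP_Weapon is a melee weapon actor that detects hits on enemy characters and stores health damage, stun damage and stamina cost stats.
; Attack clears the hit-actor list, so each actor is processed only once per attack.
; DetectHit sphere-traces Pawns between the weapon mesh's start and end sockets.
; New hits on a BP_Character from a different CharacterGroup call its combat component's OnHit, without passing the stats.
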(event Custom|DetectHit
  (params (CharacterGroup :type E_CharacterGroup%20Enum :default "NewEnumerator0"))
  (bind _weaponmesh (Variables|Default|GetWeaponMesh))
  (bind _outhits (Collision|MultiSphereTraceForObjects (Transformation|GetSocketLocation _weaponmesh "start") (Transformation|GetSocketLocation _weaponmesh "end") 25.0 (Utilities|Array|MakeArray "ObjectTypeQuery3") false 0 "None"))
  (bind _array_element (Utilities|Array|ForEachLoopwithBreak _outhits)
    (:LoopBody
      (if (not (Utilities|Array|ContainsItem (Variables|Default|GetHitAtctors) (.hitactor _array_element)))
        (Utilities|Array|Add (Variables|Default|GetHitAtctors) (.hitactor _array_element))
        (bind _asbp_character (Utilities|Casting|CastToBP_Character (.hitactor _array_element)))
        (if (Utilities|Enum|NotEqual(Enum) (Variables|/Game/Project/Blueprints/Characters/BP_Character.BP_Character_C|GetCharacterGroup _asbp_character) CharacterGroup)
          (Default|OnHit (Variables|/Game/Project/Blueprints/Characters/BP_Character.BP_Character_C|GetBP_CombatComponent _asbp_character)))))))

(event Custom|Attack
  (Utilities|Array|Clear (Variables|Default|GetHitAtctors)))

(event EventBeginPlay)

(event Collision|EventActorBeginOverlap
  (params (OtherActor :type Actor%20Object%20Reference)))

(event EventTick
  (params (DeltaSeconds :type Float%20%28single-precision%29)))

(fn ConstructionScript)

(fn SetWeaponStats
  (params (HealthDamage :type Float%20%28double-precision%29) (StunDamage :type Float%20%28double-precision%29) (StaminaCost :type Float%20%28double-precision%29))
  (Variables|Default|SetHealthDamage HealthDamage)
  (Variables|Default|SetStunDamage StunDamage)
  (Variables|Default|SetStaminaCost StaminaCost))

(fn GetWeaponStats
  (return (Variables|Default|GetHealthDamage) (Variables|Default|GetStunDamage) (Variables|Default|GetStaminaCost)))