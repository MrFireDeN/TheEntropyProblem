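; Sword weapon Blueprint that specializes a parent weapon class with its own stats and combo rules.
; BeginPlay sets health and stun damage, stamina cost and attack rate.
; ComboHandle extends the parent by advancing the step for the last attack type: two or more quick steps set the strong step to one, and strong attacks reset the quick step.
; Nodes assigning quick and strong slash montages are unconnected and never run.
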(event EventBeginPlay
  (|CallParentFunction)
  (CallFunction|SetWeaponStats 6e+01 2e+01 5.0 1.0))

(event Collision|EventActorBeginOverlap
  (params (OtherActor :type Actor%20Object%20Reference))
  (|CallParentFunction OtherActor) ; This node is disabled and will not be called.\nDrag off pins to build functionality.
)

(event EventTick
  (params (DeltaSeconds :type Float%20%28single-precision%29))
  (|CallParentFunction DeltaSeconds) ; This node is disabled and will not be called.\nDrag off pins to build functionality.
)

(fn ConstructionScript
  (|CallParentFunction))

(fn ComboHandle
  (|CallParentFunction)
  (switch Utilities|FlowControl|Switch|SwitchonE_AttackType (Variables|Default|GetLastAttackType)
    (:NewEnumerator0
      (bind _result (Math|Integer|IncrementInt (.QuickComboStep (CallFunction|GetComboSteps)))
        (:%20%20
          (CallFunction|SetQuickComboStep _result)
          (if (>= _result 2)
            (CallFunction|SetStrongComboStep 1)
            (else
              (CallFunction|SetStrongComboStep))))))
    (:NewEnumerator1
      (bind _result_2 (Math|Integer|IncrementInt (.StrongComboStep (CallFunction|GetComboSteps)))
        (:%20%20
          (CallFunction|SetStrongComboStep _result_2)
          (CallFunction|SetQuickComboStep))))))