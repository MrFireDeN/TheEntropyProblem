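; BP_Dagger is a dagger weapon Blueprint that configures a parent weapon class with dagger-specific combat data.
; On BeginPlay it runs the parent logic, then sets damage, stun, stamina cost and attack rate.
; It also assigns separate quick and strong attack montage lists, built from sword slash animations.
; It adds no other active logic, as overlap and tick events are disabled and construction only calls the parent.
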(event EventBeginPlay
  (|CallParentFunction)
  (CallFunction|SetWeaponStats 8e+01 35.0 15.0 0.5)
  (CallFunction|SetQuickAttackAnims (Utilities|Array|MakeArray "/Game/Project/Animations/Mixamo/SwordSlash/Straight_Sword_Inward_Slash_Montage.Straight_Sword_Inward_Slash_Montage" "/Game/Project/Animations/Mixamo/SwordSlash/Straight_Sword_Outward_Slash_Montage.Straight_Sword_Outward_Slash_Montage" "/Game/Project/Animations/Mixamo/SwordSlash/Half_Backhand_Sword_Inward_Slash_Montage.Half_Backhand_Sword_Inward_Slash_Montage" "/Game/Project/Animations/Mixamo/SwordSlash/Half_Backhand_Sword_Outward_Slash_Montage.Half_Backhand_Sword_Outward_Slash_Montage" "/Game/Project/Animations/Mixamo/SwordSlash/Half_Downhand_Sword_Inward_Slash_Montage.Half_Downhand_Sword_Inward_Slash_Montage"))
  (CallFunction|SetStrongAttackAnims (Utilities|Array|MakeArray "/Game/Project/Animations/Mixamo/SwordSlash/Backhand_Sword_Outward_Slash_Montage.Backhand_Sword_Outward_Slash_Montage" "/Game/Project/Animations/Mixamo/SwordSlash/Downhand_Sword_Outward_Slash_Montage.Downhand_Sword_Outward_Slash_Montage")))

(event Collision|EventActorBeginOverlap
  (params (OtherActor :type Actor%20Object%20Reference))
  (|CallParentFunction OtherActor) ; This node is disabled and will not be called.\nDrag off pins to build functionality.
)

(event EventTick
  (params (DeltaSeconds :type Float%20%28single-precision%29))
  (|CallParentFunction DeltaSeconds) ; This node is disabled and will not be called.\nDrag off pins to build functionality.
)

(fn ConstructionScript
  (|CallParentFunction))