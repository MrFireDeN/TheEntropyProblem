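; Game mode Blueprint that tracks the player's last checkpoint and handles respawning there.
; On BeginPlay it creates a note widget and binds to the respawn event on the player's BPDeathComponent.
; A new checkpoint plays a camera shutter sound and briefly shows a Russian save-point message through a retriggerable delay.
; RespawnPlayer teleports the player to the saved checkpoint's Position transform, if one is valid.
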(event Custom|SetNewCheckPoint
  (params (NewCheckpoint :type BP%20Checkpoint%20Object%20Reference))
  (if (!= NewCheckpoint (Variables|Default|GetLastCheckpoint))
    (Variables|Default|SetLastCheckpoint NewCheckpoint)
    (Audio|PlaySound2D "/Engine/VREditor/Sounds/UI/Camera_Shutter.Camera_Shutter" 1.0 1.0 0.0 0 0)
    (Utilities|SendMessage)))

(event Custom|RespawnPlayer
  (bind _lastcheckpoint (Variables|Default|GetLastCheckpoint))
  (bind _position (Variables|/Game/Project/Blueprints/Levels/BP_Checkpoint.BP_Checkpoint_C|GetPosition _lastcheckpoint))
  (bind _returnvalue (Transformation|GetWorldTransform _position))
  (Utilities|IsValid (Variables|Default|GetLastCheckpoint)
    (:Is%20Valid
      (Transformation|SetActorLocationAndRotation (Variables|Default|GetAs%20BP%20Player) (.location _returnvalue) (.rotation _returnvalue) false true))))

(event EventBeginPlay
  (bind _returnvalue (UserInterface|CreateWidget "/Game/Project/UI/WBP_Note.WBP_Note_C"))
  (Variables|Default|SetMessageWidget _returnvalue)
  (bind _asbp_player (Utilities|Casting|CastToBP_Player (Game|GetPlayerCharacter 0)))
  (bind _output_get (Variables|Default|SetAs%20BP%20Player _asbp_player))
  (EventDispatchers|BindEventtoOnPlayerRespawn (Variables|/Game/Project/Blueprints/Characters/BP_Character.BP_Character_C|GetBP_DeathComponent _output_get) (EventDispatchers|CreateEvent :!event Custom|RespawnPlayer)))

(fn ConstructionScript)