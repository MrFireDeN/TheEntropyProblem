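; BP_Health is a reusable health Blueprint that tracks current and maximum health, with functions for damage, healing and alive checks.
; TakeDamage and Heal both route through SetHealth, which clamps the value between zero and MaxHealth and returns the new health and alive state.
; SetMaxHealth accepts only positive values and does not re-clamp current health.
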(fn SetHealth
  (params (Health :type Float%20%28double-precision%29))
  (bind _output_get (Variables|Default|SetHealth (Math|Float|Clamp(Float) Health 0.0 (Variables|Default|GetMaxHealth))))
  (return _output_get (CallFunction|IsAlive)))

(fn TakeDamage
  (params (Damage :type Float%20%28double-precision%29))
  (bind (_newhealth _isalive) (CallFunction|SetHealth (- (Variables|Default|GetHealth) Damage)))
  (return _newhealth _isalive))

(fn IsAlive
  (return (> (Variables|Default|GetHealth) 0.0)))

(fn Heal
  (params (HealPoints :type Float%20%28double-precision%29))
  (bind (_newhealth _isalive) (CallFunction|SetHealth (+ (Variables|Default|GetHealth) HealPoints)))
  (return _newhealth _isalive))

(fn SetMaxHealth
  (params (MaxHealth :type Float%20%28double-precision%29))
  (if (> MaxHealth 0.0)
    (bind _output_get (Variables|Default|SetMaxHealth MaxHealth))
    (return _output_get)))

(fn GetMaxGelth
  (return (Variables|Default|GetMaxHealth)))

(fn GetHealth
  (return (Variables|Default|GetHealth)))