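; BP_HealthBar is a Blueprint that displays a health percentage on a widget component.
; BeginPlay caches the component's WB_HealthBar widget, and SetHealth clamps the incoming value to the zero-to-one range before setting its progress bar.
; Each Tick rotates the widget with FindLookAtRotation toward the player camera, feeding only the Z of both locations rather than full positions.
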(event Custom|SetHealth
  (params (Percent :type Float%20%28double-precision%29))
  (Progress|SetPercent (Variables|/Game/Project/Blueprints/WB_HealthBar.WB_HealthBar_C|GetHealthBar (Variables|Default|GetAs%20WB%20Health%20Bar)) (Math|Float|Clamp(Float) Percent)))

(event EventTick
  (params (DeltaSeconds :type Float%20%28single-precision%29))
  (Transformation|SetWorldRotation (Variables|Default|GetHealthBarWidget) (Math|Rotator|FindLookatRotation (Math|Vector|MakeVector 0.0 0.0 (.z (Transformation|GetWorldLocation (Variables|Default|GetHealthBarWidget)))) (Math|Vector|MakeVector 0.0 0.0 (.z (Camera|GetCameraLocation (Game|GetPlayerCameraManager 0))))) false false))

(event EventBeginPlay
  (bind _aswb_health_bar (Utilities|Casting|CastToWB_HealthBar (UserInterface|GetWidget (Variables|Default|GetHealthBarWidget))))
  (Variables|Default|SetAs%20WB%20Health%20Bar _aswb_health_bar))

(fn ConstructionScript)