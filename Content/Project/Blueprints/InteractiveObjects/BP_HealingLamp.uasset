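; Healing lamp interactive object that heals the player character while its heal zone is occupied.
; BeginPlay caches the player's BP_Character, and the collision's begin and end overlaps toggle IsHealZone without checking which actor overlaps, printing Russian enter and exit messages.
; While the flag is set, Tick passes Regeneration to the character's BPInteract HealingCharacter every frame, with no delta-time scaling.
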(event OnComponentBeginOverlap(Collisison)
  (params (OverlappedComponent :type Primitive%20Component%20Object%20Reference) (OtherActor :type Actor%20Object%20Reference) (OtherComp :type Primitive%20Component%20Object%20Reference) (OtherBodyIndex :type Integer) (bFromSweep :type Boolean) (SweepResult :type Hit%20Result%20Structure%20%28by%20ref%29))
  (bind _output_get (Variables|Default|SetIsHealZone true))
  (Development|PrintString "Вы находитесь в зоне лечения"))

(event OnComponentEndOverlap(Collisison)
  (params (OverlappedComponent :type Primitive%20Component%20Object%20Reference) (OtherActor :type Actor%20Object%20Reference) (OtherComp :type Primitive%20Component%20Object%20Reference) (OtherBodyIndex :type Integer))
  (bind _output_get (Variables|Default|SetIsHealZone false))
  (Development|PrintString "Вы покинули зону лечения"))

(event EventBeginPlay
  (bind _asbp_character (Utilities|Casting|CastToBP_Character (Game|GetPlayerCharacter 0)))
  (Variables|Default|SetAs%20BP%20Character _asbp_character))

(event Collision|EventActorBeginOverlap
  (params (OtherActor :type Actor%20Object%20Reference)))

(event EventTick
  (params (DeltaSeconds :type Float%20%28single-precision%29))
  (if (Variables|Default|GetIsHealZone)
    (if true
      (Default|HealingCharacter (Variables|/Game/Project/Blueprints/Characters/BP_Character.BP_Character_C|GetBP_Interact (Variables|Default|GetAs%20BP%20Character)) (Variables|Default|GetRegeneration)))))

(fn ConstructionScript)

(fn GetIsHealZone
  (return (Variables|Default|GetIsHealZone)))