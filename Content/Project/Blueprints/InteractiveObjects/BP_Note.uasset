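; BP_Note is an interactable note that shows its text on screen when the player interacts with it.
; It creates a WBP_Note widget once on BeginPlay and reuses it.
; StartInteract toggles that widget in the viewport, filling in the note's Text when shown, and EndInteract removes it.
; CanInteract always returns true, while GetName and SetName expose the note's name.
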(event EventBeginPlay
  (bind _returnvalue (UserInterface|CreateWidget "/Game/Project/UI/WBP_Note.WBP_Note_C"))
  (Variables|Default|SetNoteWidget _returnvalue))

(event Collision|EventActorBeginOverlap
  (params (OtherActor :type Actor%20Object%20Reference)))

(event EventTick
  (params (DeltaSeconds :type Float%20%28single-precision%29)))

(event EventStartInteract
  (params (Character :type BP%20Character%20Object%20Reference))
  (if (UserInterface|Viewport|IsinViewport (Variables|Default|GetNoteWidget))
    (Widget|RemovefromParent (Variables|Default|GetNoteWidget))
    (else
      (UserInterface|Viewport|AddtoViewport (Variables|Default|GetNoteWidget) 0)
      (Variables|/Script/UMG.TextBlock|SetText (Variables|/Game/Project/UI/WBP_Note.WBP_Note_C|GetWidgetText (Variables|Default|GetNoteWidget)) (Variables|Default|GetText)))))

(event EventEndInteract
  (params (Character :type BP%20Character%20Object%20Reference))
  (Widget|RemovefromParent (Variables|Default|GetNoteWidget)))

(event EventSetName
  (params (Name :type Name :default "None"))
  (Variables|Default|SetName Name))

(fn ConstructionScript)

(fn CanInteract
  (return true))

(fn GetName
  (return (Variables|Default|GetName)))