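; BP_Box is an interactive box whose static mesh can be switched to physics simulation by interacting with it.
; BeginPlay applies the Physics flag to the mesh, and the first StartInteract sets it true through a DoOnce, printing a debug message.
; CanInteract allows interaction only while physics is off, and SetName and GetName expose the box's name.
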(event EventBeginPlay
  (Physics|SetSimulatePhysics (Variables|Debug|GetStaticMeshComponent) (Variables|Default|GetPhysics)))

(event EventSetName
  (params (Name :type Name :default "None"))
  (Variables|Default|SetName Name))

(event EventStartInteract
  (params (Character :type BP%20Character%20Object%20Reference))
  (Utilities|FlowControl|DoOnce false
    (:Completed
      (Variables|Default|SetPhysics true)
      (Development|PrintString "Физика +")
      (Physics|SetSimulatePhysics (Variables|Debug|GetStaticMeshComponent) (Variables|Default|GetPhysics)))))

(fn ConstructionScript)

(fn CanInteract
  (return (not (Variables|Default|GetPhysics))))

(fn GetName
  (return (Variables|Default|GetName)))