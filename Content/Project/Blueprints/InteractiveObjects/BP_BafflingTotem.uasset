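; BP_BafflingTotem is an interactive totem that buffs Enemy-group characters inside its sphere collision.
; On overlap, it checks for BPI_EffectsInterface, records the enemy and uses a self-re-entering DoN as a loop over tracked actors.
; The loop applies long-duration strength and max HP boosts through BPEffectsComponent.
; Leaving the sphere clears both effects, removes the enemy from the list and prints a debug name.
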(event OnComponentBeginOverlap(SphereCollision)
  (params (OverlappedComponent :type Primitive%20Component%20Object%20Reference) (OtherActor :type Actor%20Object%20Reference) (OtherComp :type Primitive%20Component%20Object%20Reference) (OtherBodyIndex :type Integer) (bFromSweep :type Boolean) (SweepResult :type Hit%20Result%20Structure%20%28by%20ref%29))
  (bind _bp_effectscomponent (Variables|Default|GetBP_EffectsComponent))
  (bind _overlapping_actors (Variables|Default|GetOverlapping%20Actors))
  (bind _returnvalue (Utilities|Array|Length _overlapping_actors))
  (if (Utilities|DoesObjectImplementInterface OtherActor "/Game/Project/Blueprints/BPI_EffectsInterface.BPI_EffectsInterface_C")
    (bind _asbp_character (Utilities|Casting|CastToBP_Character OtherActor))
    (bind _output_get (Variables|Default|SetAs%20BP%20Character _asbp_character))
    (switch Utilities|FlowControl|Switch|SwitchonE_CharacterGroup (Variables|/Game/Project/Blueprints/Characters/BP_Character.BP_Character_C|GetCharacterGroup _output_get)
      (:NewEnumerator3
        (Utilities|Array|SetArrayElem _overlapping_actors _returnvalue _output_get true)
        (bind _counter (Utilities|FlowControl|DoN (+ _returnvalue 1) :!label _label)
          (:Exit
            (if (> _counter _returnvalue)
              (goto _label Reset)
              (else
                (Default|Strenght _bp_effectscomponent 5.0 999.0 (Utilities|Array|Get(acopy) _overlapping_actors (- _counter 1)))
                (Default|IncreasingtheMaxHp _bp_effectscomponent 5.0 999.0 (Utilities|Array|Get(acopy) _overlapping_actors (- _counter 1)))
                (goto _label)))))))))

(event OnComponentEndOverlap(SphereCollision)
  (params (OverlappedComponent :type Primitive%20Component%20Object%20Reference) (OtherActor :type Actor%20Object%20Reference) (OtherComp :type Primitive%20Component%20Object%20Reference) (OtherBodyIndex :type Integer))
  (if (Utilities|DoesObjectImplementInterface OtherActor "/Game/Project/Blueprints/BPI_EffectsInterface.BPI_EffectsInterface_C")
    (Development|PrintString (Utilities|GetDisplayName OtherActor))
    (bind _asbp_character (Utilities|Casting|CastToBP_Character OtherActor))
    (bind _output_get (Variables|Default|SetAs%20BP%20Character _asbp_character))
    (switch Utilities|FlowControl|Switch|SwitchonE_CharacterGroup (Variables|/Game/Project/Blueprints/Characters/BP_Character.BP_Character_C|GetCharacterGroup _output_get)
      (:NewEnumerator3
        (Default|ClearEffects (Variables|Default|GetBP_EffectsComponent) _output_get false false false true false true)
        (Utilities|Array|RemoveItem (Variables|Default|GetOverlapping%20Actors) _output_get)))))

(event EventBeginPlay)

(event Collision|EventActorBeginOverlap
  (params (OtherActor :type Actor%20Object%20Reference)))

(event EventTick
  (params (DeltaSeconds :type Float%20%28single-precision%29)))

(fn ConstructionScript)