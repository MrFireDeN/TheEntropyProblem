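; Interactive swinging door that rotates up to 90 degrees away from the player.
; Entering the collision volume enables input and calls InteractWithDoor, which opens a closed door or reverses the timeline otherwise; leaving disables input.
; Swing direction comes from the dot product of the player-to-door vector and the door's right vector.
; The timeline drives the rotation, clears the player's Interacting flag and restores the closed state after reversing.
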(event OnComponentBeginOverlap(DoorCollision)
  (params (OverlappedComponent :type Primitive%20Component%20Object%20Reference) (OtherActor :type Actor%20Object%20Reference) (OtherComp :type Primitive%20Component%20Object%20Reference) (OtherBodyIndex :type Integer) (bFromSweep :type Boolean) (SweepResult :type Hit%20Result%20Structure%20%28by%20ref%29))
  (Input|EnableInput (Game|GetPlayerController 0))
  (Variables|Default|SetOverlapCollision true)
  (CallFunction|InteractwithDoor))

(event OnComponentEndOverlap(DoorCollision)
  (params (OverlappedComponent :type Primitive%20Component%20Object%20Reference) (OtherActor :type Actor%20Object%20Reference) (OtherComp :type Primitive%20Component%20Object%20Reference) (OtherBodyIndex :type Integer))
  (Input|DisableInput (Game|GetPlayerController 0))
  (Variables|Default|SetOverlapCollision false))

(event Custom|InteractWithDoor
  (bind _door (Variables|Default|GetDoor))
  (if (Variables|Default|GetOverlapCollision)
    (if (Variables|Default|GetIsCloseDoor)
      (Variables|Default|SetDotProduct (Math|Vector|DotProduct (Math|Vector|Normalize (- (Transformation|GetWorldLocation _door) (Transformation|GetActorLocation (Variables|Default|GetAs%20BP%20Player)))) (Math|Vector|GetRightVector _door)))
      (Variables|Default|SetIsCloseDoor false)
      (bind (_direction _rotation) (Timeline|DoorRatation Play)
        (:Update
          (Transformation|SetRelativeRotation (Variables|Default|GetDoor) (Math|Rotator|MakeRotator 0.0 0.0 (Math|Float|Lerp 0.0 (Math|Float|SelectFloat 9e+01 -9e+01 (>= (Variables|Default|GetDotProduct) 0.0)) _rotation)) false false))
        (:Finished
          (switch Utilities|FlowControl|Switch|SwitchonETimelineDirection _direction
            (:Backward
              (Variables|Default|SetIsCloseDoor true)))))
      (Variables|/Game/Project/Blueprints/Characters/BP_Character.BP_Character_C|SetInteracting (Variables|Default|GetAs%20BP%20Player) false)
      (else
        (Timeline|DoorRatation Reverse)))
    (else
      (Development|PrintString "Hello"))))

(event EventBeginPlay
  (bind _asbp_character (Utilities|Casting|CastToBP_Character (Game|GetPlayerCharacter 0)))
  (Variables|Default|SetAs%20BP%20Player _asbp_character))

(event Collision|EventActorBeginOverlap
  (params (OtherActor :type Actor%20Object%20Reference)))

(event EventTick
  (params (DeltaSeconds :type Float%20%28single-precision%29)))

(event Collision|EventActorEndOverlap
  (params (OtherActor :type Actor%20Object%20Reference)))

(fn ConstructionScript)