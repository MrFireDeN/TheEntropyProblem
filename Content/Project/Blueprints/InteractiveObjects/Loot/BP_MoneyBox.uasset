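; BP_MoneyBox is an interactable money pickup that grants its stored Money amount to the character who interacts with it.
; StartInteract calls AddMoney on that character's BPMoneyComponent, then destroys the box.
; CanInteract always returns true, while GetName and SetName read and write the box's Name.
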(event EventSetName
  (params (Name :type Name :default "None"))
  (Variables|Default|SetName Name))

(event EventStartInteract
  (params (Character :type BP%20Character%20Object%20Reference))
  (Default|AddMoney (Variables|/Game/Project/Blueprints/Characters/BP_Character.BP_Character_C|GetBP_MoneyComponent Character) (Variables|Default|GetMoney))
  (Actor|DestroyActor))

(fn ConstructionScript)

(fn CanInteract
  (return true))

(fn GetName
  (return (Variables|Default|GetName)))