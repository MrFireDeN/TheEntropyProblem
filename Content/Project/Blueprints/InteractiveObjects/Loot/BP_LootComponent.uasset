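; BP_LootComponent is a component that spawns loot around its owning actor when SpawnLoot is called.
; It walks the Loots array in order, rolling each entry's Chance independently and picking the first that passes, so earlier entries take priority.
; A BP_MoneyBox pick spawns once with Count as its Money; other valid classes spawn Count times.
; Each spawn is randomly offset horizontally from the owner.
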(event Custom|SpawnLoot
  ;[1 1 1] Spawn Loot
  (bind _output_get (Variables|Default|SetLoot%20to%20Spawn (CallFunction|LoottoSpawn)))
  (if (== (.object _output_get) "/Game/Project/Blueprints/InteractiveObjects/Loot/BP_MoneyBox.BP_MoneyBox_C")
    (bind _actor (Utilities|SpawnActor))
    (bind _asbp_money_box (Utilities|Casting|CastToBP_MoneyBox _actor))
    (Variables|/Game/Project/Blueprints/InteractiveObjects/Loot/BP_MoneyBox.BP_MoneyBox_C|SetMoney _asbp_money_box (Class|KismetMathLibrary|ToInt64(Integer) (.count (Variables|Default|GetLoot%20to%20Spawn))))
    (elif (Utilities|IsValidClass (.object _output_get))
      (for _index (range 1 (.count _output_get))
        (Utilities|SpawnActor)))))

(event EventBeginPlay
  (Variables|Default|SetOwner (Components|GetOwner)))

(fn LoottoSpawn
  (bind _array_element (Utilities|Array|ForEachLoopwithBreak (Variables|Default|GetLoots) :!label _label)
    (:LoopBody
      (if (> (.Chance (Utilities|Struct|BreakS_Loot _array_element)) (Math|Random|RandomFloat))
        (Utilities|FlowControl|Sequence
          (:then_0
            (goto _label Break))
          (:then_1
            (return _array_element)))))))