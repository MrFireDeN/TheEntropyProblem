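; BP_DialogueAI is an AI controller that runs dialogue sequences as behavior trees.
; It creates a dialogue UI widget at BeginPlay and runs DialogueTree when dialogue starts.
; Ending dialogue stops the brain component, removes the widget from its parent and clears its line list.
; The widget is not added to the screen in this Blueprint.
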(event Custom|StartDialogue
  (AI|RunBehaviorTree (Variables|Default|GetDialogueTree)))

(event Custom|EndDialogue
  (bind _braincomponent (Variables|Default|GetBrainComponent))
  (bind _dialoguewidget (Variables|Default|GetDialogueWidget))
  (Utilities|IsValid _braincomponent
    (:Is%20Valid
      (AI|Logic|StopLogic _braincomponent "")
      (Widget|RemovefromParent _dialoguewidget)
      (Widget|Panel|ClearChildren (Variables|/Game/Project/UI/Dialogue/WBP_DialogueBox.WBP_DialogueBox_C|GetLineList (Variables|/Game/Project/UI/Dialogue/WBP_DialogueUI.WBP_DialogueUI_C|GetDialogueBox _dialoguewidget))))))

(event EventBeginPlay
  (bind _returnvalue (UserInterface|CreateWidget "/Game/Project/UI/Dialogue/WBP_DialogueUI.WBP_DialogueUI_C"))
  (Variables|Default|SetDialogueWidget _returnvalue))

(fn ConstructionScript)