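; Behavior Tree task that displays a single line of dialogue in the dialogue UI.
; It gets the dialogue widget from the Blackboard, clears its line list and adds a new line widget with the task's text.
; It also binds an event to skip-line on the player controller, then finishes successfully through FinishLine after a fixed two-second delay.
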(event Custom|FinishLine
  (AI|BehaviorTree|FinishExecute true))

(event EventReceiveExecuteAI
  (params (OwnerController :type AI%20Controller%20Object%20Reference) (ControlledPawn :type Pawn%20Object%20Reference))
  (bind _aswbp_dialogue_ui (Utilities|Casting|CastToWBP_DialogueUI (Class|BTFunctionLibrary|GetBlackboardValueasObject (Variables|Default|GetDialogueWidget))))
  (bind _output_get (Variables|Default|SetLine%20List (Variables|/Game/Project/UI/Dialogue/WBP_DialogueBox.WBP_DialogueBox_C|GetLineList (Variables|/Game/Project/UI/Dialogue/WBP_DialogueUI.WBP_DialogueUI_C|GetDialogueBox _aswbp_dialogue_ui))))
  (Widget|Panel|ClearChildren _output_get)
  (bind _returnvalue (UserInterface|CreateWidget "/Game/Project/UI/Dialogue/WBP_DilaogueLine.WBP_DilaogueLine_C" 0 (Variables|Default|GetLine)))
  (Widget|Panel|AddChild (Variables|Default|GetLine%20List) _returnvalue)
  (bind _asbp_player_controller (Utilities|Casting|CastToBP_PlayerController (Game|GetPlayerController 0)))
  (EventDispatchers|BindEventtoSkipLine _asbp_player_controller (EventDispatchers|CreateEvent :!event Custom|FinishLine))
  (Utilities|FlowControl|Delay 2.0)
  (CallFunction|FinishLine))