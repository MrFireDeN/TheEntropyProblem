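; Boss arena gate in the Forest level that wakes the boss and locks behind the player.
; When the player overlaps it with the key found and the boss still alive, it calls WakeUp on the boss.
; Ending the overlap under the same conditions switches the box collision to BlockAll.
; A Restart event restores pawn-only overlap, and BeginPlay binds a delegate to the player death component's respawn event.
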(event Custom|Restart
  (Collision|SetCollisionProfileName (Variables|Default|GetBox) "OverlapOnlyPawn" true :!class /Script/Engine.PrimitiveComponent))

(event Collision|EventActorBeginOverlap
  (params (OtherActor :type Actor%20Object%20Reference))
  (Utilities|CanStart OtherActor)
  (Default|WakeUp (Variables|Default|GetBoss)))

(event EventFindKey
  (Variables|Default|SetIsFindKey true))

(event EventBossKilled
  (Variables|Default|SetIsBossKilled true))

(event Collision|EventActorEndOverlap
  (params (OtherActor :type Actor%20Object%20Reference))
  (Utilities|CanStart OtherActor)
  (Collision|SetCollisionProfileName (Variables|Default|GetBox) "BlockAll" true :!class /Script/Engine.PrimitiveComponent))

(event EventBeginPlay
  (bind _asbp_player (Utilities|Casting|CastToBP_Player (Game|GetPlayerCharacter 0)))
  (bind _output_get (Variables|Default|SetAs%20BP%20Player _asbp_player))
  (EventDispatchers|BindEventtoOnPlayerRespawn (Variables|/Game/Project/Blueprints/Characters/BP_Character.BP_Character_C|GetBP_DeathComponent _output_get) (EventDispatchers|CreateEvent :!event Custom|Restart)))

(fn ConstructionScript)