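; BP_CityGate is an interactable city gate that sinks into the ground to open when the interacting character holds its key.
; BossKilled enables interaction and FindKey disables it; without the key, interacting briefly shows a Russian "gate is locked" message through a WBP_Note widget.
; Open and Close only set the target location, which Tick approaches smoothly with VInterpTo.
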(event Custom|Open
  (Variables|Default|SetTargetLocation (Variables|Default|GetOpenLocation)))

(event Custom|Close
  (Variables|Default|SetTargetLocation (Variables|Default|GetCloseLocation)))

(event EventBeginPlay
  (bind _returnvalue (UserInterface|CreateWidget "/Game/Project/UI/WBP_Note.WBP_Note_C"))
  (Variables|Default|SetMessageWidget _returnvalue)
  (bind _output_get (Variables|Default|SetCloseLocation (Transformation|GetActorLocation)))
  (Variables|Default|SetOpenLocation (Math|Vector|MakeVector (.x _output_get) (.y _output_get) (- (.z _output_get) 5.8e+02)))
  (CallFunction|Close))

(event EventSetName
  (params (Name :type Name :default "None"))
  (Variables|Default|SetName Name))

(event EventTick
  (params (DeltaSeconds :type Float%20%28single-precision%29))
  (if (Class|KismetMathLibrary|NotEqualExactlyVectorVector (Variables|Default|GetTargetLocation) (Transformation|GetActorLocation))
    (Transformation|SetActorLocation (Math|Interpolation|VInterpTo (Transformation|GetActorLocation) (Variables|Default|GetTargetLocation) DeltaSeconds 1.0) false false)))

(event EventBossKilled
  (Variables|Default|SetCanToInteract true))

(event EventFindKey
  (Variables|Default|SetCanToInteract false))

(event EventStartInteract
  (params (Character :type BP%20Character%20Object%20Reference))
  (if (Utilities|Array|ContainsItem (Variables|/Game/Project/Blueprints/Characters/BP_Character.BP_Character_C|GetKeys Character) (Variables|Default|GetKey))
    (CallFunction|Open)
    (else
      (Utilities|SendMessage "Ворота заперты!"))))

(fn ConstructionScript)

(fn CanInteract
  (return (Variables|Default|GetCanToInteract)))

(fn GetName
  (return (Variables|Default|GetName)))