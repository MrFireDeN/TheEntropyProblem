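; BP_ForestBoss is the Forest level's boss, which starts dormant and invisible until a FindKey event reveals it.
; On BeginPlay it runs its parent logic, calls Sleep and hides itself; FindKey only unhides it.
; When its death component fires OnBossDeath, it sends BossKilledMessage to every actor implementing BPI_ForestLevel, decoupling the boss from level-specific reactions.
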(event OnBossDeath(BP_DeathComponent)
  (bind _outactors (Actor|GetAllActorswithInterface "/Game/Project/Blueprints/Levels/Forest/BPI_ForestLevel.BPI_ForestLevel_C"))
  (for _array_element _outactors
    (Class|BPIForestLevel|BossKilled(Message) _array_element)))

(event EventBeginPlay
  (|CallParentFunction)
  (CallFunction|Sleep)
  (Rendering|SetActorHiddenInGame true))

(event Collision|EventActorBeginOverlap
  (params (OtherActor :type Actor%20Object%20Reference))
  (|CallParentFunction OtherActor) ; This node is disabled and will not be called.\nDrag off pins to build functionality.
)

(event EventTick
  (params (DeltaSeconds :type Float%20%28single-precision%29))
  (|CallParentFunction DeltaSeconds) ; This node is disabled and will not be called.\nDrag off pins to build functionality.
)

(event EventFindKey
  (Rendering|SetActorHiddenInGame false))

(fn ConstructionScript
  (|CallParentFunction))