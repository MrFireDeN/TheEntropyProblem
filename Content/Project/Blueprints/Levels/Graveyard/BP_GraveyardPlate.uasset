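; BP_GraveyardPlate is a pressure plate for the Graveyard level that signals other actors when something steps on or off it.
; On begin overlap it calls the parent handler, then sends PlatePressMessage(true) to every actor implementing BPI_Graveyard.
; End overlap sends false the same way, without a parent call.
; Neither event filters the overlapping actor or counts how many remain on the plate.
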(event EventBeginPlay
  (|CallParentFunction) ; This node is disabled and will not be called.\nDrag off pins to build functionality.
)

(event Collision|EventActorBeginOverlap
  (params (OtherActor :type Actor%20Object%20Reference))
  (|CallParentFunction OtherActor)
  (bind _outactors (Actor|GetAllActorswithInterface "/Game/Project/Blueprints/Levels/Graveyard/BPI_Graveyard.BPI_Graveyard_C"))
  (for _array_element _outactors
    (Class|BPIGraveyard|PlatePress(Message) _array_element true)))

(event EventTick
  (params (DeltaSeconds :type Float%20%28single-precision%29))
  (|CallParentFunction DeltaSeconds) ; This node is disabled and will not be called.\nDrag off pins to build functionality.
)

(event Collision|EventActorEndOverlap
  (params (OtherActor :type Actor%20Object%20Reference))
  (bind _outactors (Actor|GetAllActorswithInterface "/Game/Project/Blueprints/Levels/Graveyard/BPI_Graveyard.BPI_Graveyard_C"))
  (for _array_element _outactors
    (Class|BPIGraveyard|PlatePress(Message) _array_element false)))

(fn ConstructionScript
  (|CallParentFunction))