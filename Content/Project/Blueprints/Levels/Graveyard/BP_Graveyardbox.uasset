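; BP_Graveyardbox is an interactable box for the Graveyard level that turns physical when used and notifies other graveyard actors.
; StartInteract enables physics simulation on its static mesh, then finds every actor implementing BPI_Graveyard and sends each the BoxIteractMessage.
; The box needs no direct references to those listeners, as the interface broadcast handles the link.
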(event EventBeginPlay
  (|CallParentFunction) ; This node is disabled and will not be called.\nDrag off pins to build functionality.
)

(event Collision|EventActorBeginOverlap
  (params (OtherActor :type Actor%20Object%20Reference))
  (|CallParentFunction OtherActor) ; This node is disabled and will not be called.\nDrag off pins to build functionality.
)

(event EventTick
  (params (DeltaSeconds :type Float%20%28single-precision%29))
  (|CallParentFunction DeltaSeconds) ; This node is disabled and will not be called.\nDrag off pins to build functionality.
)

(event EventStartInteract
  (bind _output_get (Variables|Default|SetPhysics true))
  (Physics|SetSimulatePhysics (Variables|Default|GetStaticMeshComponent) _output_get)
  (bind _outactors (Actor|GetAllActorswithInterface "/Game/Project/Blueprints/Levels/Graveyard/BPI_Graveyard.BPI_Graveyard_C"))
  (for _array_element _outactors
    (Class|BPIGraveyard|BoxIteract(Message) _array_element)))

(fn ConstructionScript
  (|CallParentFunction))