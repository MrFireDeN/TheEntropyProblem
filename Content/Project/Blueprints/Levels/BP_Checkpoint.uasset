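; BP_Checkpoint is a level checkpoint that registers itself with the game mode when the player reaches it.
; On BeginPlay it caches references to BP_Gamemod and the first player's BP_Player character.
; When that cached character begins overlapping the Trigger component, the SetCheckpoint event passes the checkpoint to the game mode's SetNewCheckPoint.
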(event OnComponentBeginOverlap(Trigger)
  (params (OverlappedComponent :type Primitive%20Component%20Object%20Reference) (OtherActor :type Actor%20Object%20Reference) (OtherComp :type Primitive%20Component%20Object%20Reference) (OtherBodyIndex :type Integer) (bFromSweep :type Boolean) (SweepResult :type Hit%20Result%20Structure%20%28by%20ref%29))
  (if (== OtherActor (Variables|Default|GetAs%20BP%20Player))
    (CallFunction|SetCheckpoint)))

(event Custom|SetCheckpoint
  (Default|SetNewCheckPoint (Variables|Default|GetAs%20BP%20Gamemod) self))

(event EventBeginPlay
  (bind _asbp_gamemod (Utilities|Casting|CastToBP_Gamemod (Game|GetGameMode)))
  (Variables|Default|SetAs%20BP%20Gamemod _asbp_gamemod)
  (bind _asbp_player (Utilities|Casting|CastToBP_Player (Game|GetPlayerCharacter 0)))
  (Variables|Default|SetAs%20BP%20Player _asbp_player))

(fn ConstructionScript)