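; Health component for BP_Character owners that tracks current and maximum health.
; On BeginPlay it resets health and caches the owner's death component and status bar, plus the HUD for players.
; Damage and healing route through SetHealth, which clamps, updates bar and HUD, and triggers HandleDeath at zero, provided the bar is valid.
; Changing max health refills health and refreshes the HUD, leaving the status bar untouched.
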(event Custom|SetMaxHealth
  (params (MaxHealth :type Float%20%28double-precision%29))
  (bind _player_hud (Variables|Default|GetPlayer%20HUD))
  ;[0.1771 0.1771 0.1771] Set Max Health
  (if (> MaxHealth 0.0)
    (Variables|Default|SetMaxHealth MaxHealth)
    (CallFunction|ResetHealth)
    (Utilities|IsValid _player_hud
      (:Is%20Valid
        (Default|UpdateMaxHealth _player_hud)))
    (else
      (Development|PrintText (Utilities|Text|FormatText "Invalid Max Health Value. Your value: {MaxHealth}" MaxHealth) true true "(R=1.000000,G=0.000000,B=0.000000,A=1.000000)" 2.0 "Error"))))

(event Custom|SetHealth
  (params (Health :type Float%20%28double-precision%29))
  (bind _player_hud (Variables|Default|GetPlayer%20HUD))
  (bind _as_bp_health_bar (Variables|Default|GetAs%20BP%20Health%20Bar))
  (bind _as_bp_death_component (Variables|Default|GetAs%20BP%20Death%20Component))
  ;[0.03976 0.4167 0.07214] Set Health
  (Variables|Default|SetHealth (Math|Float|Clamp(Float) Health 0.0 (Variables|Default|GetMaxHealth)))
  ;;[1 1 1] Health Bar Handler
  (Utilities|IsValid _as_bp_health_bar
    (:Is%20Valid
      (Default|SetHealth _as_bp_health_bar (/ (Variables|Default|GetHealth) (Variables|Default|GetMaxHealth)))
      (Utilities|IsValid _player_hud
        (:Is%20Valid
          (Default|UpdateHealth _player_hud))
        (:Is%20Not%20Valid
          _))
      ;;[0.2083 0.2083 0.2083] Death Handling
      (if (not (CallFunction|IsAlive))
        (Utilities|IsValid _as_bp_death_component
          (:Is%20Valid
            (Default|HandleDeath _as_bp_death_component))
          (:Is%20Not%20Valid
            (Development|PrintText "DeathComponent Is NOT Valid" true true "(R=1.000000,G=0.000000,B=0.000000,A=1.000000)" 2.0 "Error")))))
    (:Is%20Not%20Valid
      (Development|PrintText "HealthBar Is NOT Valid" true true "(R=1.000000,G=0.000000,B=0.000000,A=1.000000)" 2.0 "Error"))))

(event Custom|TakeDamage
  (params (Damage :type Float%20%28double-precision%29))
  ;[0 0.3305 0.4427] Take Damage & Heal
  (CallFunction|SetHealth (- (Variables|Default|GetHealth) Damage)))

(event Custom|Heal
  (params (HealPoints :type Float%20%28double-precision%29))
  ;[0 0.3305 0.4427] Take Damage & Heal
  (CallFunction|SetHealth (+ (Variables|Default|GetHealth) HealPoints)))

(event Custom|ResetHealth
  (bind _player_hud (Variables|Default|GetPlayer%20HUD))
  ;[1 1 1] Reset Health
  (Variables|Default|SetHealth (Variables|Default|GetMaxHealth))
  (Utilities|IsValid _player_hud
    (:Is%20Valid
      (Default|UpdateHealth _player_hud))))

(event EventBeginPlay
  (bind _returnvalue (Components|GetOwner))
  (CallFunction|ResetHealth)
  (bind _asbp_character (Utilities|Casting|CastToBP_Character _returnvalue)
    (:then
      (Variables|Default|SetAs%20BP%20Death%20Component (Variables|/Game/Project/Blueprints/Characters/BP_Character.BP_Character_C|GetBP_DeathComponent _asbp_character))
      (bind _asbp_status_bar (Utilities|Casting|CastToBP_StatusBar (Variables|/Script/Engine.ChildActorComponent|GetChildActor (Variables|/Game/Project/Blueprints/Characters/BP_Character.BP_Character_C|GetStatusBarChildActor _asbp_character))))
      (Variables|Default|SetAs%20BP%20Health%20Bar _asbp_status_bar)
      ;[1 1 1] Player HUD init
      (bind _asbp_player (Utilities|Casting|CastToBP_Player _returnvalue))
      (bind _asbp_player_controller (Utilities|Casting|CastToBP_PlayerController (Pawn|GetLocalViewingPlayerController _asbp_player)))
      (bind _output_get (Variables|Default|SetPlayer%20HUD (Variables|/Game/Project/Blueprints/BP_PlayerController.BP_PlayerController_C|GetPlayerHUD _asbp_player_controller)))
      (Default|UpdateMaxHealth _output_get))
    (:CastFailed
      (Development|PrintText "Failed To Cast Character" true true "(R=1.000000,G=0.000000,B=0.000000,A=1.000000)" 2.0 "Error"))))

(fn IsAlive
  (return (> (Variables|Default|GetHealth) 0.0)))

(fn GetHealth
  (return (Variables|Default|GetHealth)))

(fn GetMaxHealth
  (return (Variables|Default|GetMaxHealth)))