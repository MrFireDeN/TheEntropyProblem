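; Stun meter component for BP_Character that immobilizes its owner when stun points fill up.
; AddStun changes the clamped point total, which Tick also adjusts over time while the character is not stunned.
; Reaching the maximum stops mesh animation and disables movement, then a one-second retriggerable delay restores walking without clearing points.
; ResetStun clears points and the stunned flag, while IsActionStunned checks a separate point threshold.
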(event Custom|AddStun
  (params (StunPoints :type Float%20%28double-precision%29))
  (CallFunction|SetStunPoints (+ (Variables|Default|GetStunPoints) StunPoints)))

(event Custom|ApplyStun
  (bind _as_bp_character (Variables|Default|GetAs%20BP%20Character))
  (bind _charactermovement (Variables|/Script/Engine.Character|GetCharacterMovement _as_bp_character))
  (Variables|Default|SetStunned true)
  (Audio|Components|Audio|Stop (Variables|/Script/Engine.Character|GetMesh _as_bp_character))
  (Pawn|Components|CharacterMovement|DisableMovement _charactermovement)
  (Utilities|FlowControl|RetriggerableDelay 1.0)
  (Variables|Default|SetStunned false)
  (Pawn|Components|CharacterMovement|SetMovementMode _charactermovement "MOVE_Walking" 0))

(event Custom|ResetStun
  (CallFunction|SetStunPoints 0.0)
  (Variables|Default|SetStunned false))

(event EventBeginPlay
  (bind _asbp_character (Utilities|Casting|CastToBP_Character (Components|GetOwner)))
  (Variables|Default|SetAs%20BP%20Character _asbp_character))

(event EventTick
  (params (DeltaSeconds :type Float%20%28single-precision%29))
  (if (not (CallFunction|IsStunned))
    (bind _result (Math|Float|NegateFloat DeltaSeconds)
      (:%20%20
        (CallFunction|AddStun _result)))))

(fn SetStunPoints
  (params (StanPoints :type Float%20%28double-precision%29))
  (bind _output_get (Variables|Default|SetStunPoints (Math|Float|Clamp(Float) StanPoints 0.0 (Variables|Default|GetMaxStunPoints))))
  (if (Math|Float|NearlyEqual(Float) _output_get (Variables|Default|GetMaxStunPoints) 0.01)
    (CallFunction|ApplyStun))
  (return _output_get))

(fn IsStunned
  (return (Variables|Default|GetStunned)))

(fn IsActionStunned
  (return (>= (Variables|Default|GetStunPoints) (Variables|Default|GetActionStunPoints))))