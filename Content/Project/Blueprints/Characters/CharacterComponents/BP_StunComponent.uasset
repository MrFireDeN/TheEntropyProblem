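; Character component that tracks stun points and stuns the owner when they reach the maximum, updating its status bar and, for players, the HUD.
; Tick drains the points unless the character is stunned or a retriggerable delay after the last added stun still blocks it.
; Stunning a living character plays a montage and disables movement until it completes or is interrupted.
; A lower action threshold is exposed as a separate query.
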(event Custom|AddStun
  (params (StunPoints :type Float%20%28double-precision%29))
  (CallFunction|SetStunPoints (+ (Variables|Default|GetStunPoints) StunPoints))
  (Variables|Default|SetStunReleaseBlock true)
  (Utilities|FlowControl|RetriggerableDelay 0.5)
  (Variables|Default|SetStunReleaseBlock false))

(event Custom|ApplyStun
  (bind _as_bp_character (Variables|Default|GetAs%20BP%20Character))
  (bind _charactermovement (Variables|/Script/Engine.Character|GetCharacterMovement _as_bp_character))
  (Utilities|CanApplyStun)
  (Animation|Montage|PlayMontage (Variables|/Script/Engine.Character|GetMesh (Variables|Default|GetAs%20BP%20Character)) "/Game/Project/Animations/Mixamo/Kneeling/AM_Stuned.AM_Stuned"
    (:then
      (Variables|Default|SetStunned true)
      (Audio|Components|Audio|Stop (Variables|/Script/Engine.Character|GetMesh _as_bp_character))
      (Pawn|Components|CharacterMovement|SetMovementMode _charactermovement "MOVE_None" 0))
    (:OnCompleted
      (Variables|Default|SetStunned false :!label _label)
      (Pawn|Components|CharacterMovement|SetMovementMode _charactermovement "MOVE_Walking" 0))
    (:OnInterrupted
      (goto _label))))

(event Custom|ResetStun
  (CallFunction|SetStunPoints 0.0)
  (Variables|Default|SetStunned false))

(event EventBeginPlay
  (bind _returnvalue (Components|GetOwner))
  (bind _asbp_character (Utilities|Casting|CastToBP_Character _returnvalue))
  (Variables|Default|SetAs%20BP%20Character _asbp_character)
  (bind _asbp_status_bar (Utilities|Casting|CastToBP_StatusBar (Variables|/Script/Engine.ChildActorComponent|GetChildActor (Variables|/Game/Project/Blueprints/Characters/BP_Character.BP_Character_C|GetStatusBarChildActor _asbp_character))))
  (Variables|Default|SetAs%20BP%20Stun%20Bar _asbp_status_bar)
  ;[1 1 1] Player HUD init
  (bind _asbp_player (Utilities|Casting|CastToBP_Player _returnvalue))
  (bind _asbp_player_controller (Utilities|Casting|CastToBP_PlayerController (Pawn|GetLocalViewingPlayerController _asbp_player)))
  (bind _output_get (Variables|Default|SetPlayer%20HUD (Variables|/Game/Project/Blueprints/BP_PlayerController.BP_PlayerController_C|GetPlayerHUD _asbp_player_controller)))
  (Default|UpdateMaxStun _output_get))

(event EventTick
  (params (DeltaSeconds :type Float%20%28single-precision%29))
  (Utilities|CanReleaseStun)
  (CallFunction|SetStunPoints (- (Variables|Default|GetStunPoints) (* DeltaSeconds (Variables|Default|GetStunReleaseSpeed)))))

(fn SetStunPoints
  (params (StanPoints :type Float%20%28double-precision%29))
  (bind _player_hud (Variables|Default|GetPlayer%20HUD))
  (bind _output_get (Variables|Default|SetStunPoints (Math|Float|Clamp(Float) StanPoints 0.0 (Variables|Default|GetMaxStunPoints))))
  (Default|SetStun (Variables|Default|GetAs%20BP%20Stun%20Bar) (/ _output_get (Variables|Default|GetMaxStunPoints)))
  (Utilities|IsValid _player_hud
    (:Is%20Valid
      (Default|UpdateStun _player_hud))
    (:Is%20Not%20Valid
      _))
  (if (Math|Float|NearlyEqual(Float) (Variables|Default|GetStunPoints) (Variables|Default|GetMaxStunPoints) 0.01)
    (CallFunction|ApplyStun))
  (return (Variables|Default|GetStunPoints)))

(fn IsStunned
  (return (Variables|Default|GetStunned)))

(fn IsActionStunned
  (return (>= (Variables|Default|GetStunPoints) (Variables|Default|GetActionStunPoints))))

(fn GetStunPoints
  (return (Variables|Default|GetStunPoints)))

(fn GetMaxStunPoints
  (return (Variables|Default|GetMaxStunPoints)))