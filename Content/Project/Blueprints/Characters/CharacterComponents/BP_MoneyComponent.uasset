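; Actor component for characters that holds a money balance and exposes functions to get, set, add and take money.
; AddMoney and TakeMoney check the value, then route the balance change through SetMoney, which applies its own range check before writing the variable.
; The set, add and take functions return a success flag with an amount.
; The component has no active event logic.
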(event EventBeginPlay)

(event EventTick
  (params (DeltaSeconds :type Float%20%28single-precision%29)))

(fn AddMoney
  (params (Money :type Integer64))
  (bind _returnvalue (>= Money 0))
  (if _returnvalue
    (bind _amount (CallFunction|SetMoney (+ (Variables|Default|GetMoney) Money))))
  (return _returnvalue _amount))

(fn SetMoney
  (params (Money :type Integer64))
  (bind _returnvalue (>= Money 0))
  (if _returnvalue
    (Variables|Default|SetMoney 0))
  (return _returnvalue (Variables|Default|GetMoney)))

(fn TakeMoney
  (params (Money :type Integer64))
  (if (<= Money 0)
    (bind (_isset _amount) (CallFunction|SetMoney (- (Variables|Default|GetMoney) Money))))
  (return _isset _amount))

(fn GetMoney
  (return (Variables|Default|GetMoney)))