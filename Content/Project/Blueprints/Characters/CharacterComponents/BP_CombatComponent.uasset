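; Character combat component that handles attacks, weapon cycling, melee hit detection and hit reactions, gated by health, stamina, stun, dodge and attack-state checks.
; Attacks delegate to the child-actor weapon and drain stamina.
; DetectHit sphere-traces between weapon sockets, skips already-hit actors and same-group characters, and calls OnHit on each victim's combat component.
; OnHit drains stamina when shielding, otherwise applies health and stun damage with a random react montage.
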(event Custom|ChangeWeapon
  (bind _as_bp_character (Variables|Default|GetAs%20BP%20Character))
  (bind _weaponchildactor (Variables|/Game/Project/Blueprints/Characters/BP_Character.BP_Character_C|GetWeaponChildActor _as_bp_character))
  (Utilities|CanChangeWeapon
    (:True
      (Utilities|NextCurrentWeapon)
      (ChildActorComponent|SetChildActorClass _weaponchildactor (Utilities|Array|Get(acopy) (Variables|/Game/Project/Blueprints/Characters/BP_Character.BP_Character_C|GetCharacterWeapons (Variables|Default|GetAs%20BP%20Character)) (Variables|Default|GetCurrentWeapon)))
      (bind _asbp_base_weapon (Utilities|Casting|CastToBP_BaseWeapon (Variables|/Script/Engine.ChildActorComponent|GetChildActor _weaponchildactor)))
      (Variables|Default|SetAs%20BP%20Base%20Weapon _asbp_base_weapon))))

(event Custom|OnHit
  (params (HealthDamage :type Float%20%28double-precision%29) (StunDamage :type Float%20%28double-precision%29))
  ;[0 0.372 1] HitReact
  (Utilities|CanonHit
    (:true
      (if (Default|IsUsingShield (Variables|/Game/Project/Blueprints/Characters/BP_Character.BP_Character_C|GetBP_AbilitiesComponent (Variables|Default|GetAs%20BP%20Character)))
        (Default|TakeStamina (Variables|Default|GetBP%20Stamina%20Component) (* (+ HealthDamage StunDamage) 0.1))
        (else
          (Default|TakeDamage (Variables|Default|GetBP%20Health%20Component) HealthDamage)
          (Default|AddStun (Variables|Default|GetBP%20Stun%20Component) StunDamage)
          (Utilities|CanPlayHitAnim)
          (Animation|Montage|PlayMontage (Variables|Default|GetMesh) (Utilities|Select :Index (Math|Random|RandomIntegerinRange 0 2) :Option%200 "/Game/Project/Animations/Mixamo/Hit/standing_react_large_from_left_Montage.standing_react_large_from_left_Montage" :Option%201 "/Game/Project/Animations/Mixamo/Hit/standing_react_large_from_right_Montage.standing_react_large_from_right_Montage" :Option%202 "/Game/Project/Animations/Mixamo/Hit/standing_react_large_gut_Montage.standing_react_large_gut_Montage") 2.0
            (:then
              (Variables|Default|SetGettingHit true))
            (:OnCompleted
              (Variables|Default|SetGettingHit false :!label _label))
            (:OnInterrupted
              (goto _label))))))))

(event Custom|Attack
  (params (AttackType :type E_AttackType%20Enum :default "NewEnumerator0"))
  (bind _as_bp_base_weapon (Variables|Default|GetAs%20BP%20Base%20Weapon))
  ;[1 0.1591 0] Attack
  (Utilities|CanAttack
    (:True
      (Default|Attack _as_bp_base_weapon AttackType)
      (Default|TakeStamina (Variables|Default|GetBP%20Stamina%20Component) (.StaminaCost (Default|GetWeaponStats _as_bp_base_weapon))))))

(event Custom|DetectHit
  (bind _as_bp_base_weapon (Variables|Default|GetAs%20BP%20Base%20Weapon))
  (bind _as_bp_base_weapon_2 (Variables|Default|GetAs%20BP%20Base%20Weapon))
  (bind _as_bp_base_weapon_3 (Variables|Default|GetAs%20BP%20Base%20Weapon))
  (bind (_healthdamage _stundamage) (Default|CalculateDamage _as_bp_base_weapon))
  (bind _weaponmesh (Variables|/Game/Project/Blueprints/Weapons/BP_BaseWeapon.BP_BaseWeapon_C|GetWeaponMesh _as_bp_base_weapon_3))
  ;[0 1 0.832] HitDetect
  (bind _outhits (Collision|MultiSphereTraceForObjects (Transformation|GetSocketLocation _weaponmesh "start") (Transformation|GetSocketLocation _weaponmesh "end") (* (.x (Transformation|GetActorScale3D _as_bp_base_weapon_2)) (.AttackSphereRadius (Default|GetWeaponStats _as_bp_base_weapon_2))) (Utilities|Array|MakeArray "ObjectTypeQuery3") false 0 "None"))
  (bind _array_element (Utilities|Array|ForEachLoopwithBreak _outhits)
    (:LoopBody
      (if (not (Utilities|Array|ContainsItem (Variables|Default|GetHitActors) (.hitactor _array_element)))
        (Utilities|Array|Add (Variables|Default|GetHitActors) (.hitactor _array_element))
        (bind _asbp_character (Utilities|Casting|CastToBP_Character (.hitactor _array_element)))
        (if (Utilities|Enum|NotEqual(Enum) (Variables|/Game/Project/Blueprints/Characters/BP_Character.BP_Character_C|GetCharacterGroup _asbp_character) (Variables|/Game/Project/Blueprints/Characters/BP_Character.BP_Character_C|GetCharacterGroup (Variables|Default|GetAs%20BP%20Character)))
          (CallFunction|OnHit (Variables|/Game/Project/Blueprints/Characters/BP_Character.BP_Character_C|GetBP_CombatComponent _asbp_character) _healthdamage _stundamage))))))

(event EventBeginPlay
  (bind _asbp_character (Utilities|Casting|CastToBP_Character (Components|GetOwner)))
  (bind _output_get (Variables|Default|SetAs%20BP%20Character _asbp_character))
  (Variables|Default|SetBP%20Health%20Component (Variables|/Game/Project/Blueprints/Characters/BP_Character.BP_Character_C|GetBP_HealthComponent _output_get))
  (Variables|Default|SetBP%20Movement%20Component (Variables|/Game/Project/Blueprints/Characters/BP_Character.BP_Character_C|GetBP_MovementComponent _output_get))
  (Variables|Default|SetMesh (Variables|/Script/Engine.Character|GetMesh _output_get))
  (Variables|Default|SetBP%20Stun%20Component (Variables|/Game/Project/Blueprints/Characters/BP_Character.BP_Character_C|GetBP_StunComponent _output_get))
  (Variables|Default|SetBP%20Stamina%20Component (Variables|/Game/Project/Blueprints/Characters/BP_Character.BP_Character_C|GetBP_StaminaComponent _output_get))
  (bind _asbp_base_weapon (Utilities|Casting|CastToBP_BaseWeapon (Variables|/Script/Engine.ChildActorComponent|GetChildActor (Variables|/Game/Project/Blueprints/Characters/BP_Character.BP_Character_C|GetWeaponChildActor _output_get))))
  (Variables|Default|SetAs%20BP%20Base%20Weapon _asbp_base_weapon))

(fn AttackLock
  (params (IsLock :type Boolean))
  (Variables|Default|SetAttaking IsLock))

(fn SetAttacking
  (params (Attaking :type Boolean))
  (bind _output_get (Variables|Default|SetAttaking Attaking))
  (if (not _output_get)
    (Utilities|Array|Clear (Variables|Default|GetHitActors))))

(fn ClearHitActors
  (Utilities|Array|Clear (Variables|Default|GetHitActors)))