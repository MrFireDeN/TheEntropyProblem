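; Character component that handles death for players and other characters derived from BP_Character.
; HandleDeath plays a random death montage, disables movement and sets the capsule to probe-only collision.
; Players see a death widget and respawn after a delay with reset health at the first PlayerStart found, using a dodge montage as movement and collision are restored.
; Other characters spawn loot through their loot component and are destroyed after a delay.
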(event Custom|HandleDeath
  (Animation|Montage|PlayMontage (Variables|/Script/Engine.Character|GetMesh (Variables|Default|GetAs%20BP%20Character)) (Utilities|Select :Index (Math|Random|RandomIntegerinRange 0 7) :Option%200 "/Game/Project/Animations/Mixamo/Death/Standing_Death_Backward_01_Montage.Standing_Death_Backward_01_Montage" :Option%201 "/Game/Project/Animations/Mixamo/Death/Standing_Death_Backward_02_Montage.Standing_Death_Backward_02_Montage" :Option%202 "/Game/Project/Animations/Mixamo/Death/Standing_Death_Forward_01_Montage.Standing_Death_Forward_01_Montage" :Option%203 "/Game/Project/Animations/Mixamo/Death/Standing_Death_Forward_02_Montage.Standing_Death_Forward_02_Montage" :Option%204 "/Game/Project/Animations/Mixamo/Death/Standing_Death_Left_01_Montage.Standing_Death_Left_01_Montage" :Option%205 "/Game/Project/Animations/Mixamo/Death/Standing_Death_Forward_02_Montage.Standing_Death_Forward_02_Montage" :Option%206 "/Game/Project/Animations/Mixamo/Death/Standing_Death_Right_01_Montage.Standing_Death_Right_01_Montage" :Option%207 "/Game/Project/Animations/Mixamo/Death/Standing_Death_Right_02_Montage.Standing_Death_Right_02_Montage")
    (:then
      (Pawn|Components|CharacterMovement|DisableMovement (Variables|/Script/Engine.Character|GetCharacterMovement (Variables|Default|GetAs%20BP%20Character)))
      (Collision|SetCollisionEnabled (Variables|/Script/Engine.Character|GetCapsuleComponent (Variables|Default|GetAs%20BP%20Character)) "ProbeOnly")
      (Utilities|Casting|CastToBP_Player (Variables|Default|GetAs%20BP%20Character)
        (:then
          ;[1 1 1] Player Death Handle
          (bind _returnvalue (UserInterface|CreateWidget "/Game/Project/UI/WBP_Death.WBP_Death_C"))
          (bind _output_get (Variables|Default|SetDeathText _returnvalue))
          (UserInterface|Viewport|AddtoViewport _output_get 0)
          (Utilities|FlowControl|Delay 3.0)
          (CallFunction|RespawnPlayer))
        (:CastFailed
          ;[1 1 1] Character Death Handle
          (Default|SpawnLoot (Variables|Default|GetBP%20Loot%20Component))
          (Utilities|FlowControl|Delay 5.0)
          (Actor|DestroyActor (Variables|Default|GetAs%20BP%20Character)))))))

(event Custom|RespawnPlayer
  (Default|ResetHealth (Variables|/Game/Project/Blueprints/Characters/BP_Character.BP_Character_C|GetBP_HealthComponent (Variables|Default|GetAs%20BP%20Character)))
  (bind _outactors (Actor|GetAllActorsOfClass "/Script/Engine.PlayerStart"))
  (Utilities|IsValid (Utilities|Array|Get(acopy) _outactors)
    (:Is%20Valid
      (Transformation|SetActorLocationAndRotation (Variables|Default|GetAs%20BP%20Character) (.location (Transformation|GetActorTransform (Utilities|Array|Get(acopy) _outactors))) (.rotation (Transformation|GetActorTransform (Utilities|Array|Get(acopy) _outactors))))
      (Animation|Montage|PlayMontage (Variables|/Script/Engine.Character|GetMesh (Variables|Default|GetAs%20BP%20Character)) "/Game/Project/Animations/Mixamo/AM_Dodge.AM_Dodge"
        (:then
          (Pawn|Components|CharacterMovement|SetMovementMode (Variables|/Script/Engine.Character|GetCharacterMovement (Variables|Default|GetAs%20BP%20Character)) "MOVE_Walking" 0)
          (Collision|SetCollisionEnabled (Variables|/Script/Engine.Character|GetCapsuleComponent (Variables|Default|GetAs%20BP%20Character)) "QueryAndPhysics")
          (Widget|RemovefromParent (Variables|Default|GetDeathText)))))))

(event EventBeginPlay
  (bind _asbp_character (Utilities|Casting|CastToBP_Character (Components|GetOwner)))
  (bind _output_get (Variables|Default|SetAs%20BP%20Character _asbp_character))
  (Variables|Default|SetBP%20Loot%20Component (Variables|/Game/Project/Blueprints/Characters/BP_Character.BP_Character_C|GetBP_LootComponent _output_get)))