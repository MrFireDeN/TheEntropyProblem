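; Character component that applies timed status effects: poison, regeneration, slowing, strength, weakness and increased max HP.
; Poison and regeneration tick each second via delay loops into the health component.
; The others scale movement, weapon or max-health values by level, then restore stored bases after retriggerable delays.
; Strength and Weakness share one active flag, blocking overlap; ClearEffects re-invokes selected effects with tiny level and short duration.
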(event Custom|Regeneration
  (params (Level :type Float%20%28double-precision%29) (Time :type Float%20%28double-precision%29) (Character :type BP%20Character%20Object%20Reference))
  (Variables|Default|SetCharacter Character)
  (Variables|Default|SetIsRegeneration true)
  (Variables|Default|SetCount 0)
  (Default|Heal (Variables|/Game/Project/Blueprints/Characters/BP_Character.BP_Character_C|GetBP_HealthComponent (Variables|Default|GetCharacter)) (* Level 2) :!label _label)
  (if (Variables|Default|GetIsRegeneration) :!label _label_2
    (if (> (Variables|Default|GetCount) Time)
      (Variables|Default|SetCount 0)
      (Variables|Default|SetIsRegeneration false)
      (goto _label_2)
      (else
        (Utilities|FlowControl|Delay 1.0)
        (Variables|Default|SetCount (+ (Variables|Default|GetCount) 1))
        (Development|PrintString "Time:")
        (Development|PrintString (Utilities|String|ToString(Float) Time) true true "(R=1.000000,G=0.000000,B=0.109699,A=1.000000)")
        (goto _label)))))

(event Custom|Poison
  (params (Level :type Float%20%28double-precision%29) (Time :type Float%20%28double-precision%29) (Character :type BP%20Character%20Object%20Reference))
  (Variables|Default|SetCharacter Character)
  (Variables|Default|SetIsPoison true)
  (Variables|Default|SetCountPoison 0)
  (Default|TakeDamage (Variables|/Game/Project/Blueprints/Characters/BP_Character.BP_Character_C|GetBP_HealthComponent (Variables|Default|GetCharacter)) (* Level 2) :!label _label)
  (if (Default|IsAlive (Variables|/Game/Project/Blueprints/Characters/BP_Character.BP_Character_C|GetBP_HealthComponent (Variables|Default|GetCharacter)))
    (if (Variables|Default|GetIsPoison) :!label _label_2
      (if (> (Variables|Default|GetCountPoison) Time)
        (Variables|Default|SetCountPoison 0)
        (Variables|Default|SetIsPoison false)
        (goto _label_2)
        (else
          (Utilities|FlowControl|Delay 1.0)
          (Variables|Default|SetCountPoison (+ (Variables|Default|GetCountPoison) 1))
          (goto _label))))))

(event Custom|Slowing
  (params (Level :type Float%20%28double-precision%29) (Time :type Float%20%28double-precision%29) (Character :type BP%20Character%20Object%20Reference))
  (bind _returnvalue (* Level 0.1))
  (bind _walkspeed (Variables|Default|GetWalkSpeed))
  (bind _runspeed (Variables|Default|GetRunSpeed))
  (bind _returnvalue_2 (* _walkspeed _returnvalue))
  (bind _returnvalue_3 (- _walkspeed _returnvalue_2))
  (Variables|Default|SetCharacter Character)
  (Development|PrintString (Utilities|String|ToString(Float) _returnvalue_3))
  (Default|SetWalkSpeed (Variables|/Game/Project/Blueprints/Characters/BP_Character.BP_Character_C|GetBP_MovementComponent (Variables|Default|GetCharacter)) _returnvalue_3)
  (Default|SetRunSpeed (Variables|/Game/Project/Blueprints/Characters/BP_Character.BP_Character_C|GetBP_MovementComponent (Variables|Default|GetCharacter)) (- _runspeed (* _runspeed (* Level 0.1))))
  (Default|SetRunning (Variables|/Game/Project/Blueprints/Characters/BP_Character.BP_Character_C|GetBP_MovementComponent (Variables|Default|GetCharacter)) false)
  (Utilities|FlowControl|RetriggerableDelay Time)
  (Default|SetWalkSpeed (Variables|/Game/Project/Blueprints/Characters/BP_Character.BP_Character_C|GetBP_MovementComponent (Variables|Default|GetCharacter)) (Variables|Default|GetWalkSpeed))
  (Default|SetRunSpeed (Variables|/Game/Project/Blueprints/Characters/BP_Character.BP_Character_C|GetBP_MovementComponent (Variables|Default|GetCharacter)) (Variables|Default|GetRunSpeed))
  (Default|SetRunning (Variables|/Game/Project/Blueprints/Characters/BP_Character.BP_Character_C|GetBP_MovementComponent (Variables|Default|GetCharacter)) false))

(event Custom|Strenght
  (params (Level :type Float%20%28double-precision%29) (Time :type Float%20%28double-precision%29) (Character :type BP%20Character%20Object%20Reference))
  (bind _returnvalue (* Level 0.1))
  (bind _output_get (Variables|Default|SetCharacter Character))
  (bind _asbp_base_weapon (Utilities|Casting|CastToBP_BaseWeapon (Variables|/Script/Engine.ChildActorComponent|GetChildActor (Variables|/Game/Project/Blueprints/Characters/BP_Character.BP_Character_C|GetWeaponChildActor _output_get))))
  (Variables|Default|SetAs%20BP%20Base%20Weapon _asbp_base_weapon)
  (if (Variables|Default|GetisFirstIter)
    (Variables|Default|SetisFirstIter false)
    (Variables|Default|SetHealth%20Damage (.HealthDamage (Default|GetWeaponStats (Variables|Default|GetAs%20BP%20Base%20Weapon))))
    (Variables|Default|SetStun%20Damage (.StunDamage (Default|GetWeaponStats (Variables|Default|GetAs%20BP%20Base%20Weapon))))
    (Variables|Default|SetStamina%20Cost (.StaminaCost (Default|GetWeaponStats (Variables|Default|GetAs%20BP%20Base%20Weapon))))
    (Variables|Default|SetAttack%20Rate (.AttackRate (Default|GetWeaponStats (Variables|Default|GetAs%20BP%20Base%20Weapon)))))
  (if (not (Variables|Default|GetIsStrenght))
    (Variables|Default|SetIsStrenght true)
    (Default|SetStats (Variables|Default|GetAs%20BP%20Base%20Weapon) (+ (.HealthDamage (Default|GetWeaponStats (Variables|Default|GetAs%20BP%20Base%20Weapon))) (* (.HealthDamage (Default|GetWeaponStats (Variables|Default|GetAs%20BP%20Base%20Weapon))) _returnvalue)) (+ (.StunDamage (Default|GetWeaponStats (Variables|Default|GetAs%20BP%20Base%20Weapon))) (* (.StunDamage (Default|GetWeaponStats (Variables|Default|GetAs%20BP%20Base%20Weapon))) _returnvalue)) (.StaminaCost (Default|GetWeaponStats (Variables|Default|GetAs%20BP%20Base%20Weapon))) (.AttackRate (Default|GetWeaponStats (Variables|Default|GetAs%20BP%20Base%20Weapon))) (.AttackSphereRadius (Default|GetWeaponStats (Variables|Default|GetAs%20BP%20Base%20Weapon))))
    (Development|PrintString (Utilities|String|ToString(Float) (.HealthDamage (Default|GetWeaponStats (Variables|Default|GetAs%20BP%20Base%20Weapon)))))
    (Utilities|FlowControl|RetriggerableDelay Time)
    (Variables|Default|SetIsStrenght false)
    (Default|SetStats (Variables|Default|GetAs%20BP%20Base%20Weapon) (Variables|Default|GetHealth%20Damage) (Variables|Default|GetStun%20Damage) (Variables|Default|GetStamina%20Cost) (Variables|Default|GetAttack%20Rate) (.AttackSphereRadius (Default|GetWeaponStats (Variables|Default|GetAs%20BP%20Base%20Weapon))))
    (Development|PrintString (Utilities|String|ToString(Float) (Variables|Default|GetHealth%20Damage)))))

(event Custom|ClearEffects
  (params (Character :type BP%20Character%20Object%20Reference) (Poison :type Boolean) (Regeneration :type Boolean) (Slowing :type Boolean) (Strenght :type Boolean) (Weakness :type Boolean) (IncreasintTheMaxHP :type Boolean))
  (Variables|Default|SetCharacter Character)
  (if Poison
    (CallFunction|Poison 0.1 1.0 (Variables|Default|GetCharacter)))
  (if Regeneration
    (CallFunction|Regeneration 0.1 1.0 (Variables|Default|GetCharacter)))
  (if Slowing
    (CallFunction|Slowing 0.1 1.0 (Variables|Default|GetCharacter)))
  (if Strenght
    (CallFunction|Strenght 0.1 1.0 (Variables|Default|GetCharacter)))
  (if Weakness
    (CallFunction|Weakness 0.1 1.0 (Variables|Default|GetCharacter)))
  (if IncreasintTheMaxHP
    (CallFunction|IncreasingtheMaxHp 0.1 1.0 (Variables|Default|GetCharacter))))

(event Custom|Weakness
  (params (Level :type Float%20%28double-precision%29) (Time :type Float%20%28double-precision%29) (Character :type BP%20Character%20Object%20Reference))
  (bind _returnvalue (* Level 0.1))
  (bind _output_get (Variables|Default|SetCharacter Character))
  (bind _asbp_base_weapon (Utilities|Casting|CastToBP_BaseWeapon (Variables|/Script/Engine.ChildActorComponent|GetChildActor (Variables|/Game/Project/Blueprints/Characters/BP_Character.BP_Character_C|GetWeaponChildActor _output_get))))
  (Variables|Default|SetAs%20BP%20Base%20Weapon _asbp_base_weapon)
  (if (Variables|Default|GetisFirstIter)
    (Variables|Default|SetisFirstIter false)
    (Variables|Default|SetHealth%20Damage (.HealthDamage (Default|GetWeaponStats (Variables|Default|GetAs%20BP%20Base%20Weapon))))
    (Variables|Default|SetStun%20Damage (.StunDamage (Default|GetWeaponStats (Variables|Default|GetAs%20BP%20Base%20Weapon))))
    (Variables|Default|SetStamina%20Cost (.StaminaCost (Default|GetWeaponStats (Variables|Default|GetAs%20BP%20Base%20Weapon))))
    (Variables|Default|SetAttack%20Rate (.AttackRate (Default|GetWeaponStats (Variables|Default|GetAs%20BP%20Base%20Weapon)))))
  (Development|PrintString (Utilities|String|ToString(Float) (.HealthDamage (Default|GetWeaponStats (Variables|Default|GetAs%20BP%20Base%20Weapon)))))
  (if (not (Variables|Default|GetIsStrenght))
    (Variables|Default|SetIsStrenght true)
    (Default|SetStats (Variables|Default|GetAs%20BP%20Base%20Weapon) (- (.HealthDamage (Default|GetWeaponStats (Variables|Default|GetAs%20BP%20Base%20Weapon))) (* (.HealthDamage (Default|GetWeaponStats (Variables|Default|GetAs%20BP%20Base%20Weapon))) _returnvalue)) (- (.StunDamage (Default|GetWeaponStats (Variables|Default|GetAs%20BP%20Base%20Weapon))) (* (.StunDamage (Default|GetWeaponStats (Variables|Default|GetAs%20BP%20Base%20Weapon))) _returnvalue)) (.StaminaCost (Default|GetWeaponStats (Variables|Default|GetAs%20BP%20Base%20Weapon))) (.AttackRate (Default|GetWeaponStats (Variables|Default|GetAs%20BP%20Base%20Weapon))) (.AttackSphereRadius (Default|GetWeaponStats (Variables|Default|GetAs%20BP%20Base%20Weapon))))
    (Utilities|FlowControl|RetriggerableDelay Time)
    (Variables|Default|SetIsStrenght false)
    (Default|SetStats (Variables|Default|GetAs%20BP%20Base%20Weapon) (Variables|Default|GetHealth%20Damage) (Variables|Default|GetStun%20Damage) (Variables|Default|GetStamina%20Cost) (Variables|Default|GetAttack%20Rate) (.AttackSphereRadius (Default|GetWeaponStats (Variables|Default|GetAs%20BP%20Base%20Weapon))))
    (Development|PrintString (Utilities|String|ToString(Float) (Variables|Default|GetHealth%20Damage)))))

(event Custom|IncreasingTheMaxHp
  (params (Level :type Float%20%28double-precision%29) (Time :type Float%20%28double-precision%29) (Character :type BP%20Character%20Object%20Reference))
  (bind _output_get (Variables|Default|SetCharacter Character))
  (if (Variables|Default|GetIsSetMaxHp)
    _
    (else
      (bind _output_get_2 (Variables|Default|SetMax%20Health (Default|GetMaxHealth (Variables|/Game/Project/Blueprints/Characters/BP_Character.BP_Character_C|GetBP_HealthComponent _output_get))))
      (Variables|Default|SetIsSetMaxHp true)))
  (Default|SetMaxHealth (Variables|/Game/Project/Blueprints/Characters/BP_Character.BP_Character_C|GetBP_HealthComponent _output_get) (+ _output_get_2 (* _output_get_2 (* Level 0.1))))
  (Development|PrintString (Utilities|String|ToString(Float) (+ _output_get_2 (* _output_get_2 (* Level 0.1)))))
  (Utilities|FlowControl|RetriggerableDelay Time)
  (Default|SetMaxHealth (Variables|/Game/Project/Blueprints/Characters/BP_Character.BP_Character_C|GetBP_HealthComponent _output_get) (Variables|Default|GetMax%20Health))
  (Development|PrintString (Utilities|String|ToString(Float) (Variables|Default|GetMax%20Health))))

(event EventBeginPlay)

(event EventTick
  (params (DeltaSeconds :type Float%20%28single-precision%29)))

(fn CastBPCharacter
  (params (Object :type Object%20Object%20Reference))
  (bind _asbp_character (Utilities|Casting|CastToBP_Character Object))
  (bind _output_get (Variables|Default|SetAs%20BP%20Character _asbp_character))
  (return _output_get))