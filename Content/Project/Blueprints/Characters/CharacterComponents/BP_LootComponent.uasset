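; BP_LootComponent is an actor component that spawns loot around its owning actor when SpawnLoot is called.
; LootToSpawn walks the Loots array in order and returns the first entry passing its random Chance roll, so earlier entries take priority.
; SpawnLoot spawns that entry's class Count times at random horizontal offsets near the owner.
; Validity, class and count each call LootToSpawn separately, so their rolls can differ.
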(event Custom|SpawnLoot
  (bind _loottospawn (CallFunction|LoottoSpawn))
  ;[1 1 1] Spawn Loot
  (if (Utilities|IsValidClass (.object _loottospawn))
    (Variables|Default|SetActorToSpawn (.object _loottospawn))
    (for _index (range 1 (.count _loottospawn))
      (Game|SpawnActorfromClass (Variables|Default|GetActorToSpawn) (Math|Transform|MakeTransform (+ (Transformation|GetActorLocation (Variables|Default|GetOwner)) (Math|Random|RandomPointinBoundingBox "0, 0, 0" "50.000000,50.000000,0.000000")) "0, 0, 0" "1.000000,1.000000,1.000000") "Undefined" "MultiplyWithRoot" 0 0))))

(event EventBeginPlay
  (Variables|Default|SetOwner (Components|GetOwner)))

(fn LoottoSpawn
  (bind _array_element (Utilities|Array|ForEachLoopwithBreak (Variables|Default|GetLoots) :!label _label)
    (:LoopBody
      (if (> (.Chance (Utilities|Struct|BreakS_Loot _array_element)) (Math|Random|RandomFloat))
        (Utilities|FlowControl|Sequence
          (:then_0
            (goto _label Break))
          (:then_1
            (return _array_element)))))))