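; Character component that handles walk/run speed and dodge rolls for BP_Character, with stamina costs.
; Tick interpolates max walk speed toward a target, drains stamina while running and drops to walk when stamina runs out.
; Dodge requires being alive, not already dodging and having stamina, then applies a velocity impulse scaled by target speed.
; Directional input plays a roll montage; no input plays a backward dodge.
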(event Custom|SetWalkSpeed
  (params (WalkSpeed :type Float%20%28double-precision%29))
  ;[1 1 1] Set Walk Speed
  (if (> WalkSpeed 0.0)
    (Variables|Default|SetWalkSpeed WalkSpeed)
    (else
      (Development|PrintText (Utilities|Text|FormatText "Invalid Speed Value. Your value: {Value}" WalkSpeed) true true "(R=1.000000,G=0.000000,B=0.000000,A=1.000000)" 2.0 "Error"))))

(event Custom|SetRunSpeed
  (params (RunSpeed :type Float%20%28double-precision%29))
  ;[1 1 1] Set Run Speed
  (if (> RunSpeed 0.0)
    (Variables|Default|SetRunSpeed RunSpeed)
    (else
      (Development|PrintText (Utilities|Text|FormatText "Invalid Speed Value. Your value: {Value}" RunSpeed) true true "(R=1.000000,G=0.000000,B=0.000000,A=1.000000)" 2.0 "Error"))))

(event Custom|Dodge
  (params (Direction :type Vector) (IsRun :type Boolean))
  ;[1 1 1] Dodging/Rolling
  (Utilities|CanDodge
    (:True
      (bind (_direction _isroll) (Utilities|CalculateDodgeVector Direction))
      (Utilities|ResetCharacterRotationandVelocity)
      (Physics|AddImpulse (Variables|Default|GetCharacter%20Movement) _direction true)
      (Animation|Montage|PlayMontage (Variables|/Script/Engine.Character|GetMesh (Variables|Default|GetAs%20BP%20Character)) (select _isroll "/Game/Project/Animations/Mixamo/AM_Sprinting_Forward_Roll.AM_Sprinting_Forward_Roll" "/Game/Project/Animations/Mixamo/AM_Dodge.AM_Dodge")
        (:then
          (Variables|Default|SetIsDodge true)
          (Default|TakeStamina (Variables|Default|GetBP%20Stamina%20Component) 1e+01))
        (:OnCompleted
          (Variables|Default|SetIsDodge false :!label _label))
        (:OnInterrupted
          (goto _label))))))

(event Custom|SetRunning
  (params (IsRun :type Boolean))
  ;[1 1 1] Set Running
  (if IsRun
    (Variables|Default|SetTargetSpeed (Variables|Default|GetRunSpeed))
    (else
      (Variables|Default|SetTargetSpeed (Variables|Default|GetWalkSpeed)))))

(event EventBeginPlay
  ;[1 1 1] Init
  (bind _asbp_character (Utilities|Casting|CastToBP_Character (Components|GetOwner)))
  (bind _output_get (Variables|Default|SetAs%20BP%20Character _asbp_character))
  (Variables|Default|SetCharacter%20Movement (Variables|/Script/Engine.Character|GetCharacterMovement _output_get))
  (Variables|Default|SetTargetSpeed (Variables|Default|GetWalkSpeed))
  (Variables|Default|SetBP%20Combat%20Component (Variables|/Game/Project/Blueprints/Characters/BP_Character.BP_Character_C|GetBP_CombatComponent _output_get))
  (Variables|Default|SetBP%20Stamina%20Component (Variables|/Game/Project/Blueprints/Characters/BP_Character.BP_Character_C|GetBP_StaminaComponent _output_get)))

(event EventTick
  (params (DeltaSeconds :type Float%20%28single-precision%29))
  ;[1 1 1] Running Handle
  (Utilities|SetSpeed DeltaSeconds)
  (Utilities|IsRunning
    (:true
      (Default|TakeStamina (Variables|Default|GetBP%20Stamina%20Component) (* DeltaSeconds 5.0))
      (if (Default|IsStaminaOut (Variables|Default|GetBP%20Stamina%20Component))
        (Variables|Default|SetTargetSpeed (Variables|Default|GetWalkSpeed))))))

(fn GetIsDodge
  (return (Variables|Default|GetIsDodge)))