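; BP_CameraMask is a player component for masking walls between the camera and character, but that logic is currently disconnected.
; BeginPlay caches the BP_Player owner's capsule, camera and mesh; Tick does nothing.
; The unused graph sphere-traces from camera to above the mesh origin, tracking blockers in a Wall array.
; It toggles their Mask material parameter through dynamic instances, restoring walls that no longer block.
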(event EventTick
  (params (DeltaSeconds :type Float%20%28single-precision%29)))

(event EventBeginPlay
  (bind _asbp_player (Utilities|Casting|CastToBP_Player (Components|GetOwner)))
  (Variables|Default|SetCapsule%20Component (Variables|/Script/Engine.Character|GetCapsuleComponent _asbp_player))
  (Variables|Default|SetCamera (Variables|/Game/Project/Blueprints/Characters/BP_Player.BP_Player_C|GetCamera _asbp_player))
  (Variables|Default|SetMesh (Variables|/Script/Engine.Character|GetMesh _asbp_player)))