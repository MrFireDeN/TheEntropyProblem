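; Stamina component for BP_Character owners that regenerates stamina on Tick, gated by exhaustion and recent-use blocks.
; TakeStamina spends points and pauses regeneration with a one-second retriggerable delay.
; All changes pass through a clamped setter that updates the HUD for players and triggers StaminaOut near zero.
; StaminaOut zeroes walk speed without restoring it here and raises a timed exhaustion flag, exposed through IsStaminaOut.
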(event Custom|StaminaOut
  ;[1 1 1] Stamine Out
  (Variables|Default|SetStaminaOutBlock true)
  (Variables|/Script/Engine.CharacterMovementComponent|SetMaxWalkSpeed (Variables|Default|GetCharacter%20Movement) 0.0)
  (Utilities|FlowControl|RetriggerableDelay 1.0)
  (Variables|Default|SetStaminaOutBlock false))

(event Custom|TakeStamina
  (params (StaminaPoints :type Float%20%28double-precision%29))
  ;[1 1 1] Take Stamina
  (CallFunction|SetStaminaPoints (- (Variables|Default|GetStaminaPoints) StaminaPoints))
  (Variables|Default|SetStaminaReleaseBlock true)
  (Utilities|FlowControl|RetriggerableDelay 1.0)
  (Variables|Default|SetStaminaReleaseBlock false))

(event EventBeginPlay
  (bind _returnvalue (Components|GetOwner))
  (bind _asbp_character (Utilities|Casting|CastToBP_Character _returnvalue))
  (Variables|Default|SetMesh (Variables|/Script/Engine.Character|GetMesh _asbp_character))
  (Variables|Default|SetCharacter%20Movement (Variables|/Script/Engine.Character|GetCharacterMovement _asbp_character))
  ;[1 1 1] Player HUD init
  (bind _asbp_player (Utilities|Casting|CastToBP_Player _returnvalue))
  (bind _asbp_player_controller (Utilities|Casting|CastToBP_PlayerController (Pawn|GetLocalViewingPlayerController _asbp_player)))
  (bind _output_get (Variables|Default|SetPlayer%20HUD (Variables|/Game/Project/Blueprints/BP_PlayerController.BP_PlayerController_C|GetPlayerHUD _asbp_player_controller)))
  (Default|UpdateMaxStamina _output_get))

(event EventTick
  (params (DeltaSeconds :type Float%20%28single-precision%29))
  ;[1 1 1] Set Stamina Point
  (Utilities|CanStaminaRelease)
  (CallFunction|SetStaminaPoints (+ (Variables|Default|GetStaminaPoints) (* DeltaSeconds (Variables|Default|GetStaminaReleaseSpeed)))))

(fn SetStaminaPoints
  (params (StaminaPoints :type Float%20%28double-precision%29))
  (bind _player_hud (Variables|Default|GetPlayer%20HUD))
  (bind _output_get (Variables|Default|SetStaminaPoints (Math|Float|Clamp(Float) StaminaPoints 0.0 (Variables|Default|GetStaminaMaxPoints))))
  (Utilities|IsValid _player_hud
    (:Is%20Valid
      (Default|UpdateStamina _player_hud))
    (:Is%20Not%20Valid
      _))
  (if (Math|Float|NearlyEqual(Float) _output_get 0.0 0.01)
    (CallFunction|StaminaOut)))

(fn IsStaminaOut
  (return (Variables|Default|GetStaminaOutBlock)))

(fn GetStaminaPoints
  (return (Variables|Default|GetStaminaPoints)))

(fn GetStaminaMaxPoints
  (return (Variables|Default|GetStaminaMaxPoints)))