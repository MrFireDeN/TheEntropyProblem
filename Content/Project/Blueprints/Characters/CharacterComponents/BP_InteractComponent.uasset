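; Character component that tracks one interactable actor for its owning BP_Character, shows an F-key prompt and triggers interaction.
; SetInteractableActor accepts an actor only when no target is held and BPI_InteractInterface allows it, then displays WBP_Interact with its name from BPI_NameInterface or display name.
; Interact sends StartInteractMessage to the target and hides the prompt.
; ClearInteractableActor sends EndInteractMessage, releases the matching target and removes the prompt.
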(event Custom|Clear%20Interactable%20Actor
  (params (Actor :type Actor%20Object%20Reference))
  ;[1 1 1] Clear Interactable Actor
  (if (== Actor (Variables|Default|GetInteractable%20Actor))
    (Class|BPIInteractInterface|EndInteract(Message) (Variables|Default|GetInteractable%20Actor) (Variables|Default|GetAs%20BP%20Character))
    (Variables|Default|SetInteractable%20Actor 0)
    (Widget|RemovefromParent (Variables|Default|GetInteract%20Widget))))

(event Custom|Set%20Interactable%20Actor
  (params (Actor :type Actor%20Object%20Reference))
  ;[1 1 1] Set Interactable Actor
  (Utilities|IsValid (Variables|Default|GetInteractable%20Actor)
    (:Is%20Not%20Valid
      (if (Utilities|DoesObjectImplementInterface Actor "/Game/Project/Blueprints/BPI_InteractInterface.BPI_InteractInterface_C")
        (bind _caninteract (Class|BPIInteractInterface|CanInteract(Message) Actor))
        (if _caninteract
          (bind _output_get (Variables|Default|SetInteractable%20Actor Actor))
          (Variables|/Script/UMG.TextBlock|SetText (Variables|/Game/Project/UI/WBP_Interact.WBP_Interact_C|GetIntaractText (Variables|Default|GetInteract%20Widget)) (Utilities|Text|FormatText "(F) Взаимодействовать с {name}" (CallFunction|GetName _output_get)))
          (UserInterface|Viewport|AddtoViewport (Variables|Default|GetInteract%20Widget) 0))))))

(event Custom|Interact
  (bind _interactable_actor (Variables|Default|GetInteractable%20Actor))
  ;[1 1 1] Interact
  (Utilities|IsValid _interactable_actor
    (:Is%20Valid
      (Class|BPIInteractInterface|StartInteract(Message) _interactable_actor (Variables|Default|GetAs%20BP%20Character))
      (Widget|RemovefromParent (Variables|Default|GetInteract%20Widget)))))

(event EventBeginPlay
  (bind _returnvalue (UserInterface|CreateWidget "/Game/Project/UI/WBP_Interact.WBP_Interact_C"))
  (Variables|Default|SetInteract%20Widget _returnvalue)
  (bind _asbp_character (Utilities|Casting|CastToBP_Character (Components|GetOwner)))
  (Variables|Default|SetAs%20BP%20Character _asbp_character))

(fn GetName
  (params (Actor :type Actor%20Object%20Reference))
  (bind _output_get (LocalVariables|SetLocalActor Actor))
  (if (Utilities|DoesObjectImplementInterface _output_get "/Game/Project/Blueprints/BPI_NameInterface.BPI_NameInterface_C")
    (bind _name (Class|BPINameInterface|GetName(Message) (LocalVariables|GetLocalActor)))
    (return _name)
    (else
      (return (Utilities|String|StringToName (Utilities|GetDisplayName (LocalVariables|GetLocalActor)))))))