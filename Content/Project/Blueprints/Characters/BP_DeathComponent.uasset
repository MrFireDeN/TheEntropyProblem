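; Death component for characters that plays a death animation, then either resets the game or removes the character.
; BeginPlay caches the owning BP_Character.
; HandleDeath plays a randomly selected directional standing death montage on its mesh, without regard to hit direction.
; After fixed delays that start alongside the montage, a BP_Player opens L_Main, while any other character is destroyed.
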(event Custom|HandleDeath
  (Animation|Montage|PlayMontage (Variables|/Script/Engine.Character|GetMesh (Variables|Default|GetAs%20BP%20Character)) (Utilities|Select :Index (Math|Random|RandomIntegerinRange 0 7) :Option%200 "/Game/Project/Animations/Mixamo/Death/Standing_Death_Backward_01_Montage.Standing_Death_Backward_01_Montage" :Option%201 "/Game/Project/Animations/Mixamo/Death/Standing_Death_Backward_02_Montage.Standing_Death_Backward_02_Montage" :Option%202 "/Game/Project/Animations/Mixamo/Death/Standing_Death_Forward_01_Montage.Standing_Death_Forward_01_Montage" :Option%203 "/Game/Project/Animations/Mixamo/Death/Standing_Death_Forward_02_Montage.Standing_Death_Forward_02_Montage" :Option%204 "/Game/Project/Animations/Mixamo/Death/Standing_Death_Left_01_Montage.Standing_Death_Left_01_Montage" :Option%205 "/Game/Project/Animations/Mixamo/Death/Standing_Death_Forward_02_Montage.Standing_Death_Forward_02_Montage" :Option%206 "/Game/Project/Animations/Mixamo/Death/Standing_Death_Right_01_Montage.Standing_Death_Right_01_Montage" :Option%207 "/Game/Project/Animations/Mixamo/Death/Standing_Death_Right_02_Montage.Standing_Death_Right_02_Montage")
    (:then
      (Utilities|Casting|CastToBP_Player (Variables|Default|GetAs%20BP%20Character)
        (:then
          (Utilities|FlowControl|Delay 3.0)
          (Game|OpenLevel(byName) "L_Main"))
        (:CastFailed
          (Utilities|FlowControl|Delay 5.0)
          (Actor|DestroyActor (Variables|Default|GetAs%20BP%20Character)))))))

(event EventBeginPlay
  (bind _asbp_character (Utilities|Casting|CastToBP_Character (Components|GetOwner)))
  (Variables|Default|SetAs%20BP%20Character _asbp_character))