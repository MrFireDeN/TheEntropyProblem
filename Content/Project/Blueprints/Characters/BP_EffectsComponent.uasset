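; Effects component that applies timed Poison, Regeneration, Slowing, Strenght and Weakness effects, each scaled by Level, to player 0's character.
; BeginPlay caches that character and its child-actor weapon.
; Poison and Regeneration tick each second through delay loops sharing one counter, driving the health component.
; Slowing temporarily changes movement speeds; Strenght and Weakness share a guard flag, temporarily scale weapon damage, then restore first-use cached stats.
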(event Custom|Regeneration
  (params (Level :type Integer) (Time :type Integer))
  (Variables|Default|SetIsRegeneration true)
  (Default|Heal (Variables|/Game/Project/Blueprints/Characters/BP_Character.BP_Character_C|GetBP_HealthComponent (Variables|Default|GetAs%20BP%20Character)) (Math|Conversions|ToFloat(Integer) (* Level 2)) :!label _label)
  (if (Variables|Default|GetIsRegeneration) :!label _label_2
    (if (> (Variables|Default|GetCount) Time)
      (Variables|Default|SetCount 0)
      (Variables|Default|SetIsRegeneration false)
      (goto _label_2)
      (else
        (Utilities|FlowControl|Delay 1.0)
        (Variables|Default|SetCount (+ (Variables|Default|GetCount) 1))
        (goto _label)))))

(event Custom|Poison
  (params (Level :type Integer) (Time :type Integer))
  (bind _as_bp_character (Variables|Default|GetAs%20BP%20Character))
  (bind _bp_healthcomponent (Variables|/Game/Project/Blueprints/Characters/BP_Character.BP_Character_C|GetBP_HealthComponent _as_bp_character))
  (Variables|Default|SetIsPoison true)
  (Default|TakeDamage _bp_healthcomponent (Math|Conversions|ToFloat(Integer) (* Level 2)) :!label _label)
  (if (Default|IsAlive _bp_healthcomponent)
    (if (Variables|Default|GetIsPoison) :!label _label_2
      (if (> (Variables|Default|GetCount) Time)
        (Variables|Default|SetCount 0)
        (Variables|Default|SetIsPoison false)
        (goto _label_2)
        (else
          (Utilities|FlowControl|Delay 1.0)
          (Variables|Default|SetCount (+ (Variables|Default|GetCount) 1))
          (goto _label))))))

(event Custom|Slowing
  (params (Level :type Float%20%28double-precision%29) (Time :type Float%20%28double-precision%29))
  (bind _returnvalue (* Level 0.1))
  (bind _returnvalue_2 (* Level 0.1))
  (bind _as_bp_character (Variables|Default|GetAs%20BP%20Character))
  (bind _bp_movementcomponent (Variables|/Game/Project/Blueprints/Characters/BP_Character.BP_Character_C|GetBP_MovementComponent _as_bp_character))
  (Default|SetWalkSpeed _bp_movementcomponent (- (* (Variables|Default|GetWalkSpeed) _returnvalue) _returnvalue))
  (Default|SetRunSpeed _bp_movementcomponent (- (* (Variables|Default|GetRunSpeed) _returnvalue_2) _returnvalue_2))
  (Default|SetRunning _bp_movementcomponent true)
  (Utilities|FlowControl|Delay Time)
  (Default|SetWalkSpeed _bp_movementcomponent (Variables|Default|GetWalkSpeed))
  (Default|SetRunSpeed _bp_movementcomponent (Variables|Default|GetRunSpeed))
  (Default|SetRunning _bp_movementcomponent true))

(event Custom|Strenght
  (params (Level :type Float%20%28double-precision%29) (Time :type Float%20%28double-precision%29))
  (bind _returnvalue (* Level 0.1))
  (bind _as_bp_base_weapon (Variables|Default|GetAs%20BP%20Base%20Weapon))
  (bind _as_bp_base_weapon_2 (Variables|Default|GetAs%20BP%20Base%20Weapon))
  (bind (_healthdamage _stundamage _staminacost _attackrate) (Default|GetWeaponStats _as_bp_base_weapon))
  (bind (_healthdamage_2 _stundamage_2 _staminacost_2 _attackrate_2) (Default|GetWeaponStats _as_bp_base_weapon_2))
  (if (Variables|Default|GetisFirstIter)
    (Variables|Default|SetisFirstIter false)
    (Variables|Default|SetHealth%20Damage _healthdamage_2)
    (Variables|Default|SetStun%20Damage _stundamage_2)
    (Variables|Default|SetStamina%20Cost _staminacost_2)
    (Variables|Default|SetAttack%20Rate _attackrate_2))
  (Development|PrintString (Utilities|String|ToString(Float) _healthdamage_2))
  (if (not (Variables|Default|GetIsStrenght))
    (Variables|Default|SetIsStrenght true)
    (Default|SetStats _as_bp_base_weapon (+ _healthdamage (* _healthdamage _returnvalue)) (+ _stundamage (* _stundamage _returnvalue)) _staminacost _attackrate)
    (Utilities|FlowControl|Delay Time)
    (Variables|Default|SetIsStrenght false)
    (Default|SetStats (Variables|Default|GetAs%20BP%20Base%20Weapon) (Variables|Default|GetHealth%20Damage) (Variables|Default|GetStun%20Damage) (Variables|Default|GetStamina%20Cost) (Variables|Default|GetAttack%20Rate))
    (Development|PrintString (Utilities|String|ToString(Float) (Variables|Default|GetHealth%20Damage)))))

(event Custom|Weakness
  (params (Level :type Float%20%28double-precision%29) (Time :type Float%20%28double-precision%29))
  (bind _returnvalue (* Level 0.1))
  (bind _as_bp_base_weapon (Variables|Default|GetAs%20BP%20Base%20Weapon))
  (bind _as_bp_base_weapon_2 (Variables|Default|GetAs%20BP%20Base%20Weapon))
  (bind (_healthdamage _stundamage _staminacost _attackrate) (Default|GetWeaponStats _as_bp_base_weapon_2))
  (bind (_healthdamage_2 _stundamage_2 _staminacost_2 _attackrate_2) (Default|GetWeaponStats _as_bp_base_weapon))
  (if (Variables|Default|GetisFirstIter)
    (Variables|Default|SetisFirstIter false)
    (Variables|Default|SetHealth%20Damage _healthdamage)
    (Variables|Default|SetStun%20Damage _stundamage)
    (Variables|Default|SetStamina%20Cost _staminacost)
    (Variables|Default|SetAttack%20Rate _attackrate))
  (Development|PrintString (Utilities|String|ToString(Float) _healthdamage))
  (if (not (Variables|Default|GetIsStrenght))
    (Variables|Default|SetIsStrenght true)
    (Default|SetStats _as_bp_base_weapon (- _healthdamage_2 (* _healthdamage_2 _returnvalue)) (- _stundamage_2 (* _stundamage_2 _returnvalue)) _staminacost_2 _attackrate_2)
    (Utilities|FlowControl|Delay Time)
    (Variables|Default|SetIsStrenght false)
    (Default|SetStats (Variables|Default|GetAs%20BP%20Base%20Weapon) (Variables|Default|GetHealth%20Damage) (Variables|Default|GetStun%20Damage) (Variables|Default|GetStamina%20Cost) (Variables|Default|GetAttack%20Rate))
    (Development|PrintString (Utilities|String|ToString(Float) (Variables|Default|GetHealth%20Damage)))))

(event EventBeginPlay
  ;[1 1 1] Cast Character
  (bind _asbp_character (Utilities|Casting|CastToBP_Character (Game|GetPlayerCharacter 0)))
  (bind _output_get (Variables|Default|SetAs%20BP%20Character _asbp_character))
  (bind _asbp_base_weapon (Utilities|Casting|CastToBP_BaseWeapon (Variables|/Script/Engine.ChildActorComponent|GetChildActor (Variables|/Game/Project/Blueprints/Characters/BP_Character.BP_Character_C|GetWeaponChildActor _output_get))))
  (Variables|Default|SetAs%20BP%20Base%20Weapon _asbp_base_weapon))

(event EventTick
  (params (DeltaSeconds :type Float%20%28single-precision%29)))