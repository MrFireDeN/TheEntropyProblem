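; BP_Character is a character Blueprint that wires up health, interaction and a key inventory.
; On BeginPlay it sets max health on BPHealthComponent and resets current health.
; Capsule overlap begin and end events pass the other actor to BPInteract to set or clear the interactable actor.
; GetKeys exposes the character's Keys variable.
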(event OnComponentEndOverlap(CapsuleComponent)
  (params (OverlappedComponent :type Primitive%20Component%20Object%20Reference) (OtherActor :type Actor%20Object%20Reference) (OtherComp :type Primitive%20Component%20Object%20Reference) (OtherBodyIndex :type Integer))
  (Default|ClearInteractableActor (Variables|Default|GetBP_Interact) OtherActor))

(event OnComponentBeginOverlap(CapsuleComponent)
  (params (OverlappedComponent :type Primitive%20Component%20Object%20Reference) (OtherActor :type Actor%20Object%20Reference) (OtherComp :type Primitive%20Component%20Object%20Reference) (OtherBodyIndex :type Integer) (bFromSweep :type Boolean) (SweepResult :type Hit%20Result%20Structure%20%28by%20ref%29))
  (Default|SetInteractableActor (Variables|Default|GetBP_Interact) OtherActor))

(event EventBeginPlay
  (bind _bp_healthcomponent (Variables|Default|GetBP_HealthComponent))
  (Default|SetMaxHealth _bp_healthcomponent 1e+02)
  (Default|ResetHealth _bp_healthcomponent))

(fn ConstructionScript)

(fn GetKeys
  (return (Variables|Default|GetKeys)))