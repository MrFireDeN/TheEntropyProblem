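; Interactive character Blueprint that lets an NPC hold a dialogue driven by its own DialogueTree.
; On BeginPlay it casts its AI controller to BP_DialogueAI, caches it and hands it the tree.
; StartInteract and EndInteract forward to that controller to start and end the dialogue, while CanInteract always returns true.
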(event EventBeginPlay
  (|CallParentFunction)
  (bind _asbp_dialogue_ai (Utilities|Casting|CastToBP_DialogueAI (AI|GetAIController self)))
  (bind _output_get (Variables|Default|SetAs%20BP%20Dialogue%20AI _asbp_dialogue_ai))
  (Variables|/Game/Project/Blueprints/Dialogue/BP_DialogueAI.BP_DialogueAI_C|SetDialogueTree _output_get (Variables|Default|GetDialogueTree)))

(event Collision|EventActorBeginOverlap
  (params (OtherActor :type Actor%20Object%20Reference)))

(event EventTick
  (params (DeltaSeconds :type Float%20%28single-precision%29)))

(event EventStartInteract
  (params (Character :type BP%20Character%20Object%20Reference))
  (Default|StartDialogue (Variables|Default|GetAs%20BP%20Dialogue%20AI)))

(event EventEndInteract
  (params (Character :type BP%20Character%20Object%20Reference))
  (Default|EndDialogue (Variables|Default|GetAs%20BP%20Dialogue%20AI)))

(fn ConstructionScript
  (|CallParentFunction))

(fn CanInteract
  (return true))