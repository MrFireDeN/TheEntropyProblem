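; Character ability component that runs the selected push, pull or shield ability, with selection and use gated by an availability array.
; Push and pull cost stamina and filter a sphere overlap to a forward cone by dot product, launching characters with a montage or applying force to static mesh actors.
; Shield toggles a flag that drains stamina on Tick until it runs out.
; Slow Down is an empty stub.
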(event Custom|UseAbility
  (bind _abilities (Variables|Default|GetAbilities))
  ;[1 1 1] Use Ability
  (switch Utilities|FlowControl|Switch|SwitchonE_Abilities (Variables|Default|GetCurrentAbility)
    (:NewEnumerator0
      (if (Utilities|Array|Get(acopy) _abilities)
        (Utilities|PushPullImpulse 1.0)))
    (:NewEnumerator1
      (if (Utilities|Array|Get(acopy) _abilities 1)
        (Utilities|PushPullImpulse -1.0)))
    (:NewEnumerator2
      (if (Utilities|Array|Get(acopy) _abilities 2)
        (Utilities|Shield)))
    (:NewEnumerator3
      (if (Utilities|Array|Get(acopy) _abilities 3)
        _))))

(event Custom|ChangeAbility
  (params (CurrentAbility :type E_Abilities%20Enum :default "NewEnumerator0"))
  ;[1 1 1] Change Ability
  (if (Utilities|Array|Get(acopy) (Variables|Default|GetAbilities) (Math|Conversions|ToInteger(Byte) CurrentAbility))
    (Variables|Default|SetCurrentAbility CurrentAbility)
    (else
      (Development|PrintText "Ability is NOT available" true true "(R=1.000000,G=0.005000,B=0.005000,A=1.000000)" 2.0 "error"))))

(event EventBeginPlay
  (bind _asbp_character (Utilities|Casting|CastToBP_Character (Components|GetOwner)))
  (bind _output_get (Variables|Default|SetAs%20BP%20Character _asbp_character))
  (Variables|Default|SetBP%20Stamina%20Component (Variables|/Game/Project/Blueprints/Characters/BP_Character.BP_Character_C|GetBP_StaminaComponent _output_get)))

(event EventTick
  (params (DeltaSeconds :type Float%20%28single-precision%29))
  (bind _bp_stamina_component (Variables|Default|GetBP%20Stamina%20Component))
  (if (Variables|Default|GetUsingShield)
    (Default|TakeStamina _bp_stamina_component DeltaSeconds)
    (if (Default|IsStaminaOut _bp_stamina_component)
      (Variables|Default|SetUsingShield false))))

(fn IsWithinCone
  (params (Target :type Actor%20Object%20Reference))
  (bind _as_bp_character (Variables|Default|GetAs%20BP%20Character))
  (return (>= (Math|Vector|DotProduct (Math|Vector|Normalize (- (Transformation|GetActorLocation Target) (Transformation|GetActorLocation _as_bp_character))) (Math|Vector|Normalize (Transformation|GetActorForwardVector _as_bp_character))) (Math|Trig|Cos(Degrees) (Variables|Default|GetAbilityRadius)))))

(fn IsUsingShield
  (return (Variables|Default|GetUsingShield)))