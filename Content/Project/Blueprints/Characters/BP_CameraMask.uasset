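; Player camera occlusion component that masks whatever blocks the camera's view of BP_Player, presumably making walls see-through.
; Every tick it sphere-traces from the camera to above the mesh origin, checking whether the capsule is hit first.
; Other hit components join a Wall array and get their "Mask" material parameter zeroed; stale entries are restored to one and removed.
; Dynamic material instances are requested on slot 0 at every update, not cached.
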(event EventTick
  (params (DeltaSeconds :type Float%20%28single-precision%29))
  (bind _outhit (Collision|SphereTraceByChannel (Transformation|GetWorldLocation (Variables|Default|GetCamera)) (+ (Transformation|GetWorldLocation (Variables|Default|GetMesh)) "0.000000,0.000000,90.000000") 3e+01 "TraceTypeQuery3" false 0 "None" false))
  (if (== (.HitComponent (Collision|BreakHitResult _outhit)) (Variables|Default|GetCapsule%20Component))
    (for _array_element (Variables|Default|GetWall)
      (bind _returnvalue (Rendering|Material|CreateDynamicMaterialInstance _array_element 0 (Rendering|Material|GetMaterial _array_element 0) "None" :!class /Script/Engine.PrimitiveComponent))
      (Rendering|Material|SetScalarParameterValue _returnvalue "Mask" 1.0 :!class /Script/Engine.MaterialInstanceDynamic)
      (Utilities|Array|Clear (Variables|Default|GetWall)))
    (else
      (Utilities|Array|Add (Variables|Default|GetWall) (.HitComponent (Collision|BreakHitResult _outhit)))
      (for _array_element_2 (Variables|Default|GetWall)
        (if (== _array_element_2 (.HitComponent (Collision|BreakHitResult _outhit)))
          (bind _returnvalue_2 (Rendering|Material|CreateDynamicMaterialInstance _array_element_2 0 (Rendering|Material|GetMaterial _array_element_2 0) "None" :!class /Script/Engine.PrimitiveComponent))
          (Rendering|Material|SetScalarParameterValue _returnvalue_2 "Mask" 0.0 :!class /Script/Engine.MaterialInstanceDynamic)
          (else
            (bind _returnvalue_3 (Rendering|Material|CreateDynamicMaterialInstance _array_element_2 0 (Rendering|Material|GetMaterial _array_element_2 0) "None" :!class /Script/Engine.PrimitiveComponent))
            (Rendering|Material|SetScalarParameterValue _returnvalue_3 "Mask" 1.0 :!class /Script/Engine.MaterialInstanceDynamic)
            (Utilities|Array|RemoveItem (Variables|Default|GetWall) _array_element_2)))))))

(event EventBeginPlay
  (bind _asbp_player (Utilities|Casting|CastToBP_Player (Components|GetOwner)))
  (Variables|Default|SetCapsule%20Component (Variables|/Script/Engine.Character|GetCapsuleComponent _asbp_player))
  (Variables|Default|SetCamera (Variables|/Game/Project/Blueprints/Characters/BP_Player.BP_Player_C|GetCamera _asbp_player))
  (Variables|Default|SetMesh (Variables|/Script/Engine.Character|GetMesh _asbp_player)))