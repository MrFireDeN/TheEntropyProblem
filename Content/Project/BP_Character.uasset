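; Character Blueprint that sets up health, tracks a nearby interactable actor and exposes a Keys value.
; On BeginPlay it sets the health component's maximum and resets health.
; Capsule overlaps store the first actor implementing BPI_InteractInterface while none is held, then send EndInteractMessage and clear it on exit.
; GetKeys returns Keys; nothing here changes that value or triggers the interaction itself.
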(event OnComponentEndOverlap(CapsuleComponent)
  (params (OverlappedComponent :type Primitive%20Component%20Object%20Reference) (OtherActor :type Actor%20Object%20Reference) (OtherComp :type Primitive%20Component%20Object%20Reference) (OtherBodyIndex :type Integer))
  (if (== OtherActor (Variables|Default|GetInteractActor))
    (Class|BPIInteractInterface|EndInteract(Message) (Variables|Default|GetInteractActor))
    (Variables|Default|SetInteractActor 0)))

(event OnComponentBeginOverlap(CapsuleComponent)
  (params (OverlappedComponent :type Primitive%20Component%20Object%20Reference) (OtherActor :type Actor%20Object%20Reference) (OtherComp :type Primitive%20Component%20Object%20Reference) (OtherBodyIndex :type Integer) (bFromSweep :type Boolean) (SweepResult :type Hit%20Result%20Structure%20%28by%20ref%29))
  (Utilities|IsValid (Variables|Default|GetInteractActor)
    (:Is%20Not%20Valid
      (if (Utilities|DoesObjectImplementInterface OtherActor "/Game/Project/Blueprints/BPI_InteractInterface.BPI_InteractInterface_C")
        (Variables|Default|SetInteractActor OtherActor)))))

(event EventBeginPlay
  (bind _bp_healthcomponent (Variables|Default|GetBP_HealthComponent))
  (Default|SetMaxHealth _bp_healthcomponent 1e+02)
  (Default|ResetHealth _bp_healthcomponent))

(fn ConstructionScript)

(fn GetKeys
  (return (Variables|Default|GetKeys)))